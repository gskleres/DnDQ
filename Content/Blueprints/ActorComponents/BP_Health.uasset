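; Health component that applies typed damage to the owner's CurrentStamina and offers clamped regeneration.
; DamageHandling (marked WIP) subtracts per-type resistance, with Meat and Shadow unresisted; only BP_HeroBase owners also get DamageSeducedEnemy and DamageMitigation.
; Mitigation drains Shield, or Resolve for Mental, then Barrier, while Shadow bypasses all pools.
; The Mental branch passes zero into ResolveProcessing instead of the incoming damage.
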(event `/Game/Blueprints/ActorComponents/BPI_DamageHandling.DamageHandling`
  (params (DamageAmount :type Integer) (DamageCauser :type "Actor Object Reference") (DamageType :type "/Game/Blueprints/ActorComponents/E_DamageType Enum" :default "NewEnumerator0"))
  ;[1 1 1] WIP - Improved Damage Handling
  (bind _asbp_hero_base (cast `/Game/Blueprints/Heroes/BP_HeroBase` (`self.GetOwner`))
    (:`then`
      (bind _damageout (`/Game/Blueprints/Heroes/BP_HeroBase.DamageSeducedEnemy` _asbp_hero_base DamageAmount))
      (bind _damageout_2 (`self.HandleResistances` _damageout DamageType))
      (bind _damageout_3 (`self.DamageMitigation` _damageout_2 DamageType))
      (`self.DamageProcessing` (`KismetMathLibrary.Conv_IntToDouble` _damageout_3)))
    (:`CastFailed`
      (bind _damageout_4 (`self.HandleResistances` DamageAmount DamageType))
      (`self.DamageProcessing` (`KismetMathLibrary.Conv_IntToDouble` _damageout_4)))))

(fn `BarrierProcessing`
  (params (DamageIn :type Integer))
  (returns (DamageOut :type Integer))
  (locals (`DamageCalculation (L)` :type Integer))
  (if (>= (`local.DamageIn`) (`self.Barrier`))
    (bind _output_get (set `local.DamageCalculation (L)` (- (`local.DamageIn`) (`self.Barrier`))))
    (set `self.Barrier` 0)
    (return _output_get)
    (else
      (set `self.Barrier` (- (`self.Barrier`) (`local.DamageIn`)))
      (return 0))))

(fn `DamageMitigation`
  (params (DamageIn :type Integer) (DamageType :type "/Game/Blueprints/ActorComponents/E_DamageType Enum" :default "NewEnumerator0"))
  (returns (DamageOut :type Integer))
  (locals (`DamageCalculation (L)` :type Integer))
  (if (`|EnumInequality` DamageType "NewEnumerator6")
    (if (`|EnumEquality` DamageType "NewEnumerator1")
      (bind _damageout (`self.ResolveProcessing` 0))
      (bind _damageout_2 (`self.BarrierProcessing` _damageout))
      (return _damageout_2)
      (else
        (bind _damageout_3 (`self.ShieldProcessing` (`local.DamageIn`)))
        (bind _damageout_4 (`self.BarrierProcessing` _damageout_3))
        (return _damageout_4)))
    (else
      (return (`local.DamageIn`)))))

(fn `DamageProcessing`
  (params (DamageAmount :type "Float (double-precision)"))
  (returns (CurrentStamina :type Integer))
  (bind _output_get (set `self.CurrentStamina` (- (`self.CurrentStamina`) (`KismetMathLibrary.Round` DamageAmount))))
  (return _output_get))

(fn `HandleResistances`
  (params (DamageIn :type Integer) (DamageType :type "/Game/Blueprints/ActorComponents/E_DamageType Enum" :default "NewEnumerator0"))
  (returns (DamageOut :type Integer))
  (locals (`CalculatedDamage (L)` :type Integer))
  (switch `/Game/Blueprints/ActorComponents/E_DamageType` DamageType
    (:`NewEnumerator0`
      _)
    (:`NewEnumerator1`
      (return (- (`local.DamageIn`) (`self.MentalResistance`))))
    (:`NewEnumerator2`
      (return (- (`local.DamageIn`) (`self.FireResistance`))))
    (:`NewEnumerator3`
      (return (- (`local.DamageIn`) (`self.IceResistance`))))
    (:`NewEnumerator4`
      (return (- (`local.DamageIn`) (`self.ShockResistance`))))
    (:`NewEnumerator5`
      (return (- (`local.DamageIn`) (`self.ToxicResistance`))))
    (:`NewEnumerator6`
      _))
  (return (`local.DamageIn`)))

(fn `Regeneration`
  (set `self.CurrentStamina` (`KismetMathLibrary.Clamp` (+ (`self.CurrentStamina`) (`self.Regenerate`)) 0 (`self.MaxStamina`))))

(fn `ResolveProcessing`
  (params (DamageIn :type Integer))
  (returns (DamageOut :type Integer))
  (locals (`DamageCalculation (L)` :type Integer))
  (if (>= (`local.DamageIn`) (`self.Resolve`))
    (bind _output_get (set `local.DamageCalculation (L)` (- (`local.DamageIn`) (`self.Resolve`))))
    (set `self.Resolve` 0)
    (return _output_get)
    (else
      (set `self.Resolve` (- (`self.Resolve`) (`local.DamageIn`)))
      (return 0))))

(fn `ShieldProcessing`
  (params (DamageIn :type Integer))
  (returns (DamageOut :type Integer))
  (locals (`DamageCalculation (L)` :type Integer))
  (if (>= (`local.DamageIn`) (`self.Shield`))
    (bind _output_get (set `local.DamageCalculation (L)` (- (`local.DamageIn`) (`self.Shield`))))
    (set `self.Shield` 0)
    (return _output_get)
    (else
      (set `self.Shield` (- (`self.Shield`) (`local.DamageIn`)))
      (return 0))))