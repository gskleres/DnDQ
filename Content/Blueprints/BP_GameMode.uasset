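; Game mode that runs a turn-based, stage-themed battle between heroes and enemies.
; BeginPlay spawns enemies on grid positions and heroes backstage from GameInstance lists and DataTables, then opens supporter selection.
; A BattleState enum tracks phases as rounds set enemy intentions, refresh hero actions and defenses, resolve enemy attacks and check win/loss or redeployment.
; Supporter abilities fire through briefly spawned actors, including a once-per-battle Twinkerbell action during cleanup.
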(event `self.ReceiveBeginPlay`
  (bind _returnvalue (`GameplayStatics.GetPlayerController` 0))
  ;[1 1 1] Begin Play
  (`WidgetBlueprintLibrary.SetInputMode_GameAndUIEx` _returnvalue null)
  (set `PlayerController.bShowMouseCursor` true _returnvalue)
  (bind _asbp_game_instance (cast `/Game/Blueprints/BP_GameInstance` (`GameplayStatics.GetGameInstance`)))
  (set `self.GameInstance` _asbp_game_instance)
  (bind _asbp_game_state (cast `/Game/Blueprints/BP_GameState` (`GameplayStatics.GetGameState`)))
  (set `self.As BP Game State` _asbp_game_state)
  (`self.AddHUD`)
  (`self.SetBattlefieldLocations`)
  (`self.SetHeroList`)
  (`self.SpawnEnemies`)
  (`self.ChooseSupporter`))

(event `SetHeroList`
  ;[1 1 1] Set Hero List
  (for _array_element (`/Game/Blueprints/BP_GameInstance.Heroes` (`self.GameInstance`))
    (if (< (`KismetArrayLibrary.Array_Length` (`self.HeroList`)) (`self.MaximumHeroes`))
      (bind _returnvalue (`|GetDataTableRow` "/Game/Blueprints/Heroes/DT_Heroes.DT_Heroes" _array_element)
        (:`then`
          (`KismetArrayLibrary.Array_Add` (`self.HeroList`) (`.ActorClass_26_AE164A27415615710C82258E2EFDB64F` (break `/Game/Blueprints/Heroes/F_HeroStats` _returnvalue)))))
      (else
        (`KismetSystemLibrary.PrintString` "Backstage Limit Reached"))))
  (`self.SetBackstageHeroCount`)
  (`self.SpawnHeroesBackstage`))

(event `SpawnEnemies`
  ;[1 1 1] Spawn Enemies at Start of Battle
  (for _array_element (`/Game/Blueprints/BP_GameInstance.Enemies` (`self.GameInstance`))
    (bind _outrownames (`DataTableFunctionLibrary.GetDataTableRowNames` "/Game/Blueprints/Enemies/DT_EnemyList.DT_EnemyList"))
    (for _array_element_2 _outrownames
      (bind _returnvalue (`|GetDataTableRow` "/Game/Blueprints/Enemies/DT_EnemyList.DT_EnemyList" _array_element_2)
        (:`then`
          (bind (_name _enemytype _blueprint) (break `/Game/Blueprints/Enemies/F_EnemyList` _returnvalue))
          (bind (_enemytype_2 _spawnlocation) (break `/Game/Blueprints/Enemies/F_SpawnList` _array_element))
          (if (`|EnumEquality` _enemytype _enemytype_2)
            (for _array_element_3 (`self.EnemyPositions`)
              (bind (_row _column) (break `/Game/Data/F_GridLocation` _spawnlocation))
              (if (and (== (`/Game/Blueprints/Battlefield/BP_EnemyPosition.Stage_Column` _array_element_3) _row) (== (`/Game/Blueprints/Battlefield/BP_EnemyPosition.Stage_Row` _array_element_3) _column))
                (bind _returnvalue_2 (`|SpawnActorFromClass` _blueprint (`KismetMathLibrary.MakeTransform` (`self.K2_GetActorLocation` _array_element_3)) "Undefined" "OverrideRootScale" null null))
                (message `/Game/Blueprints/Enemies/BPI_SetPosition.SetPosition` _returnvalue_2 _array_element_3)
                (`/Game/Blueprints/BP_GameState.AddEnemyLocation` (`self.As BP Game State`) _returnvalue_2 "NewEnumerator0" _array_element_3)))))))))

(event `BattleRoundStart`
  ;[1 1 1] Battle Round Start
  (if (not (!= (`self.BattleRound`) 0))
    (`self.SupporterBattleStart`))
  (`/Engine/EditorBlueprintResources/StandardMacros.IncrementInt` (`self.BattleRound`)
    (:`  `
      (bind _returnvalue (`|CreateWidget` "/Game/UI/WBP_RoundStart.WBP_RoundStart_C"))
      (`UserWidget.AddToViewport` _returnvalue 0)
      (`self.SetEnemyIntentions`)
      (`self.ResetHeroActions`)
      (`self.ResetShield`)
      (`self.SetShieldResolveAndBarrier`)
      (`self.IsSpotlightOccupied`)
      (`self.SupporterRoundAbility`))))

(event `ChooseSupporter`
  ;[1 1 1] Choose Supporter
  (set `self.BattleState` "NewEnumerator4")
  (bind _returnvalue (`|CreateWidget` "/Game/Blueprints/Supporters/WBP_ChooseSupporter.WBP_ChooseSupporter_C"))
  (`UserWidget.AddToViewport` _returnvalue 0)
  (`/Game/Blueprints/Supporters/WBP_ChooseSupporter.ChooseSupporter` _returnvalue))

(event `CheckEnemyPresence`
  ;[1 1 1] Check for Enemy Presence
  (`self.DoAnyEnemiesRemain`
    (:`BattleComplete`
      (bind _returnvalue (`|CreateWidget` "/Game/UI/WBP_BattleComplete.WBP_BattleComplete_C"))
      (`UserWidget.AddToViewport` _returnvalue 0))))

(event `DeployHeroesPhase`
  ;[1 1 1] Deploy Heroes Phase
  (set `self.BattleState` "NewEnumerator0"))

(event `SupporterBattleStart`
  ;[1 1 1] Supporter Battle Start
  (bind _returnvalue (`|SpawnActorFromClass` (`self.Supporter`) (`SceneComponent.K2_GetComponentToWorld` (`self.DefaultSceneRoot`)) "Undefined" "OverrideRootScale" null null))
  (`/Game/Blueprints/Supporters/BP_SupporterBase.BattleStart` _returnvalue)
  (`self.K2_DestroyActor` _returnvalue))

(event `EnemyActionPhase`
  ;[1 1 1] Enemy Actions Phase
  (set `self.HeroActionsUsed` false)
  (set `self.BattleState` "NewEnumerator2")
  (`self.PerformEnemyActions`)
  (`self.DoAnyEnemiesRemain`
    (:`Continue`
      (`self.SetBackstageHeroCount`)
      (`self.DoAnyHeroesRemain`
        (:`Continue`
          (`self.AreStagePositionsOpen`
            (:`Filled`
              (`KismetSystemLibrary.Delay` 2.0)
              (`self.EndRoundCleanup`))
            (:`Open`
              (`self.DeployHeroesPhase`))))
        (:`GameOver`
          (bind _returnvalue (`|CreateWidget` "/Game/UI/WBP_GameOver.WBP_GameOver_C"))
          (`UserWidget.AddToViewport` _returnvalue 0))))
    (:`BattleComplete`
      (`KismetSystemLibrary.PrintString` "All Enemies are Dead!"))))

(event `SupporterRoundAbility`
  ;[1 1 1] Supporter Round Start
  (bind _returnvalue (`|SpawnActorFromClass` (`self.Supporter`) (`SceneComponent.K2_GetComponentToWorld` (`self.DefaultSceneRoot`)) "Undefined" "OverrideRootScale" null null))
  (`/Game/Blueprints/Supporters/BP_SupporterBase.BattleRoundStart` _returnvalue)
  (`self.K2_DestroyActor` _returnvalue))

(event `EndRoundCleanup`
  ;[1 1 1] End Round Cleanup
  (set `self.BattleState` "NewEnumerator5")
  (bind _outactors (`GameplayStatics.GetAllActorsOfClass` "/Game/Blueprints/Heroes/BP_HeroBase.BP_HeroBase_C"))
  (for _array_element _outactors
    (if (<= (`/Game/Blueprints/ActorComponents/BP_Health.CurrentStamina` (`/Game/Blueprints/Heroes/BP_HeroBase.BP_Health` _array_element)) 0)
      (`/Game/Blueprints/Heroes/BP_HeroBase.SetPounded` _array_element)))
  (`self.TwinkerbellAction`)
  (`self.CheckStagePositions`))

(fn `AddHUD`
  (bind _returnvalue (`|CreateWidget` "/Game/UI/WBP_HeroHUD.WBP_HeroHUD_C"))
  (bind _output_get (set `self.HUD` _returnvalue))
  (`UserWidget.AddToViewport` _output_get 0))

(fn `CheckHeroActionsComplete`
  (locals (ActionPointRemaining :type Boolean))
  ;[1 1 1] Check if hero is onstage and if hero has an action point remaining. If all onstage heroes have used their action point, then the HeroActions Phase is over for this round.
  (bind _outactors (`GameplayStatics.GetAllActorsOfClass` "/Game/Blueprints/Heroes/BP_HeroBase.BP_HeroBase_C"))
  (for _array_element _outactors
    (if (`self.IsHeroOnstage` _array_element)
      (if (> (`/Game/Blueprints/Heroes/BP_HeroBase.ActionPoints` _array_element) 0)
        (set `local.ActionPointRemaining` true))))
  (if (not (`local.ActionPointRemaining`))
    (set `self.HeroActionsUsed` true)))

(fn `CheckStagePositions`
  (bind _returnvalue (`KismetArrayLibrary.Array_Length` (`self.StageLocations`)))
  (`KismetSystemLibrary.PrintString` (`KismetStringLibrary.Concat_StrStr` "Stage Locations: " (`KismetStringLibrary.Conv_IntToString` _returnvalue)) true true (struct :`G` 0.66 :`B` 1.0 :`A` 1.0) 5.0)
  (if (> _returnvalue 0)
    (`self.DeployHeroesPhase`)
    (else
      (`self.BattleRoundStart`))))

(fn `HeroRegeneration`
  (bind _outactors (`GameplayStatics.GetAllActorsOfClass` "/Game/Blueprints/Heroes/BP_HeroBase.BP_HeroBase_C"))
  (for _array_element _outactors
    (`/Game/Blueprints/ActorComponents/BP_Health.Regeneration` (`/Game/Blueprints/Heroes/BP_HeroBase.BP_Health` _array_element))))

(fn `IsHeroOnstage`
  (params (Hero :type "/Game/Blueprints/Heroes/BP_HeroBase Object Reference"))
  (returns (`On Stage` :type Boolean))
  (bind _returnvalue (`GameplayStatics.GetObjectClass` (`/Game/Blueprints/Heroes/BP_HeroBase.StageLocation` Hero)))
  (return (or (== _returnvalue "/Game/Blueprints/Battlefield/StagePositions/BP_Spotlight.BP_Spotlight_C") (== _returnvalue "/Game/Blueprints/Battlefield/StagePositions/BP_StageLeft.BP_StageLeft_C") (== _returnvalue "/Game/Blueprints/Battlefield/StagePositions/BP_StageRight.BP_StageRight_C"))))

(fn `IsSpotlightOccupied`
  (locals (IsSpotlightEmpty :type Boolean))
  (for _array_element (`self.StageLocations`)
    (bind _returnvalue (`KismetSystemLibrary.GetDisplayName` _array_element))
    (`KismetSystemLibrary.PrintString` _returnvalue)
    (bind _returnvalue_2 (`KismetStringLibrary.EqualEqual_StrStr` _returnvalue "BP_Spotlight"))
    (if _returnvalue_2
      (set `local.IsSpotlightEmpty` _returnvalue_2)))
  (if (`local.IsSpotlightEmpty`)
    (`self.DeployHeroesPhase`)
    (else
      (set `self.BattleState` "NewEnumerator1"))))

(fn `PerformEnemyActions`
  (for _array_element (`/Game/Blueprints/BP_GameState.EnemyPositions` (`self.As BP Game State`))
    (bind _asbp_enemy_base (cast `/Game/Blueprints/Enemies/BP_EnemyBase` (`.Enemy_8_0A2295EE40072C1942B114ADBC16CCE4` (break `/Game/Blueprints/Battlefield/F_EnemyPosition` _array_element))))
    (`/Game/Blueprints/Enemies/BP_EnemyBase.PerformAction` _asbp_enemy_base)))

(fn `ResetHeroActions`
  (bind _outactors (`GameplayStatics.GetAllActorsOfClass` "/Game/Blueprints/Heroes/BP_HeroBase.BP_HeroBase_C"))
  (for _array_element _outactors
    (if (and (not (`/Game/Blueprints/Heroes/BP_HeroBase.Pounded` _array_element)) (not (`/Game/Blueprints/Heroes/BP_HeroBase.Stunned` _array_element)))
      (set `/Game/Blueprints/Heroes/BP_HeroBase.ActionPoints` 1 _array_element)
      (`/Game/Blueprints/Heroes/BP_HeroBase.SetActionPointsWidget` _array_element))))

(fn `ResetShield`
  (bind _outactors (`GameplayStatics.GetAllActorsOfClass` "/Game/Blueprints/Heroes/BP_HeroBase.BP_HeroBase_C"))
  (for _array_element _outactors
    (set `/Game/Blueprints/Heroes/BP_HeroBase.Shield` 0 _array_element)
    (set `/Game/Blueprints/Heroes/BP_HeroBase.Resolve` 0 _array_element)))

(fn `SetBackstageHeroCount`
  (set `self.BackstageHeroesCount` 0)
  (bind _foundwidgets (`WidgetBlueprintLibrary.GetAllWidgetsOfClass` "/Game/UI/WBP_HeroHUD.WBP_HeroHUD_C"))
  (for _array_element _foundwidgets
    (for _array_element_2 (`PanelWidget.GetAllChildren` (`/Game/UI/WBP_HeroHUD.BackStage` _array_element))
      (bind _pounded (message `/Game/UI/HeroBackstageWidgets/BPI_Pounded.GetPounded` _array_element_2))
      (if (not _pounded)
        (`/Engine/EditorBlueprintResources/StandardMacros.IncrementInt` (`self.BackstageHeroesCount`))))))

(fn `SetBattlefieldLocations`
  (bind _outactors (`GameplayStatics.GetAllActorsOfClass` "/Game/Blueprints/Battlefield/BP_EnemyPosition.BP_EnemyPosition_C"))
  (set `self.EnemyPositions` _outactors)
  (bind _outactors_2 (`GameplayStatics.GetAllActorsOfClass` "/Game/Blueprints/Battlefield/StagePositions/BP_Spotlight.BP_Spotlight_C"))
  (set `self.StageLocations` _outactors_2)
  (bind _returnvalue (`GameplayStatics.GetActorOfClass` "/Game/Blueprints/Battlefield/StagePositions/BP_BackStage.BP_BackStage_C"))
  (set `self.Backstage` _returnvalue))

(fn `SetEnemyIntentions`
  (for _array_element (`/Game/Blueprints/BP_GameState.EnemyPositions` (`self.As BP Game State`))
    (bind _asbp_enemy_base (cast `/Game/Blueprints/Enemies/BP_EnemyBase` (`.Enemy_8_0A2295EE40072C1942B114ADBC16CCE4` (break `/Game/Blueprints/Battlefield/F_EnemyPosition` _array_element))))
    (`/Game/Blueprints/Enemies/BP_EnemyBase.ChooseAction` _asbp_enemy_base)))

(fn `SetShieldResolveAndBarrier`
  (bind _outactors (`GameplayStatics.GetAllActorsOfClass` "/Game/Blueprints/Heroes/BP_HeroBase.BP_HeroBase_C"))
  (for _array_element _outactors
    (if (`self.IsHeroOnstage` _array_element)
      (bind ((`Armor_52_EE900ED14F8100C9F60B968052DB67B2` _armor) (`Willpower_49_D4926D594885259835032AB3F760D9BA` _willpower) (`Invulnerable_47_24569B0840BBD6F6A9CD29B21F6DE344` _invulnerable)) (break `/Game/Blueprints/Heroes/F_HeroStats` (`/Game/Blueprints/Heroes/BP_HeroBase.HeroStats` _array_element)))
      (set `/Game/Blueprints/Heroes/BP_HeroBase.Shield` _armor _array_element)
      (set `/Game/Blueprints/Heroes/BP_HeroBase.Resolve` _willpower _array_element)
      (set `/Game/Blueprints/Heroes/BP_HeroBase.Barrier` _invulnerable _array_element))))

(fn `SpawnHeroesBackstage`
  (for _array_element (`self.HeroList`)
    (bind _returnvalue (`|SpawnActorFromClass` _array_element (`KismetMathLibrary.MakeTransform` (`KismetMathLibrary.MakeVector` (.x (`self.K2_GetActorLocation` (`self.Backstage`))) (.y (`self.K2_GetActorLocation` (`self.Backstage`))) (+ (.z (`self.K2_GetActorLocation` (`self.Backstage`))) 50.0))) "AdjustIfPossibleButAlwaysSpawn" "OverrideRootScale" null null))
    (message `/Game/Blueprints/Heroes/BPI_SetStageLocation.SetStageLocation` _returnvalue (`self.Backstage`))))

(fn `TwinkerbellAction`
  (if (and (== (`self.Supporter`) "/Game/Blueprints/Supporters/BP_Twinkerbell.BP_Twinkerbell_C") (not (`self.TwinkerbellUsed`)))
    (bind _returnvalue (`|SpawnActorFromClass` "/Game/Blueprints/Supporters/BP_Twinkerbell.BP_Twinkerbell_C" (`SceneComponent.K2_GetComponentToWorld` (`self.DefaultSceneRoot`)) "Undefined" "OverrideRootScale" null null))
    (`/Game/Blueprints/Supporters/BP_Twinkerbell.BringThemBitchesBack` _returnvalue)
    (`self.K2_DestroyActor` _returnvalue)
    (set `self.TwinkerbellUsed` true)
    (else
      (return))))

(fn `UserConstructionScript`)