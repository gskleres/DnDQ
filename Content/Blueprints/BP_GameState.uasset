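; Game state Blueprint that keeps a registry of where enemies stand on the stage grid.
; Events add an entry with enemy, type, column and row to EnemyPositions, or remove entries matching a given enemy while looping over that array.
; BeginPlay caches the Closet reference from the game instance held by BP_GameMode.
; An unused Debug event prints positions after a delay, re-calling itself inside its loop.
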(event `self.ReceiveBeginPlay`
  (bind _asbp_game_mode (cast `/Game/Blueprints/BP_GameMode` (`GameplayStatics.GetGameMode`)))
  (set `self.Closet` (`/Game/Blueprints/BP_GameInstance.Closet` (`/Game/Blueprints/BP_GameMode.GameInstance` _asbp_game_mode))))

(event `Debug`
  (`KismetSystemLibrary.Delay` 3.0)
  (for _array_element (`self.EnemyPositions`)
    (bind (_enemy _type _column _row) (break `/Game/Blueprints/Battlefield/F_EnemyPosition` _array_element))
    (`KismetSystemLibrary.PrintString` (`KismetStringLibrary.Concat_StrStr` (`KismetSystemLibrary.GetDisplayName` _enemy) " is in position (" (`KismetStringLibrary.Conv_IntToString` _column) "," (`KismetStringLibrary.Conv_IntToString` _row) ")"))
    (`self.Debug`)))

(event `AddEnemyLocation`
  (params (Enemy :type "Actor Object Reference") (Type :type "/Game/Blueprints/Enemies/E_EnemyList Enum" :default "NewEnumerator0") (Position :type "/Game/Blueprints/Battlefield/BP_EnemyPosition Object Reference"))
  ;[1 1 1] Add Enemy Location
  (`KismetArrayLibrary.Array_Add` (`self.EnemyPositions`) (make `/Game/Blueprints/Battlefield/F_EnemyPosition` Enemy Type (`/Game/Blueprints/Battlefield/BP_EnemyPosition.Stage_Column` Position) (`/Game/Blueprints/Battlefield/BP_EnemyPosition.Stage_Row` Position))))

(event `RemoveEnemy`
  (params (Enemy :type "/Game/Blueprints/Enemies/BP_EnemyBase Object Reference"))
  ;[1 1 1] Remove Enemy
  (for _array_element (`self.EnemyPositions`)
    (if (== (`.Enemy_8_0A2295EE40072C1942B114ADBC16CCE4` (break `/Game/Blueprints/Battlefield/F_EnemyPosition` _array_element)) Enemy)
      (`KismetArrayLibrary.Array_RemoveItem` (`self.EnemyPositions`) _array_element))))

(fn `UserConstructionScript`)