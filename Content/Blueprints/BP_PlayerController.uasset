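; Player controller for a stage-themed, turn-based hero combat game, handling click targeting and hero actions.
; A cursor trace picks tagged enemies or heroes, then dispatches Pound (front row only), Throw Shade, Seduce or Cause Drama.
; Actions, including Defend and Pull Out (backstage hero swap), work on the GameMode's active hero, mostly spending action points.
; Seduce retries d6 rolls against Chastity based on Passion, removing won enemies from the row list.
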(event `InputAction|Test`
  (params (Key :type "Key Structure"))
  (:`Pressed`
    (`KismetSystemLibrary.PrintString` "You Pressed E")))

(event `self.ReceiveBeginPlay`
  (bind _asbp_game_mode (cast `/Game/Blueprints/BP_GameMode` (`GameplayStatics.GetGameMode`)))
  (set `self.GameMode` _asbp_game_mode))

(event `InputAction|Interact`
  (params (Key :type "Key Structure"))
  ;[1 1 1] Left Mouse Button Click
  (:`Pressed`
    (if (`self.SelectingTarget`)
      (`self.SelectTarget`))))

(event `SelectTarget`
  (bind (_bblockinghit _binitialoverlap _time _distance _location _impactpoint _normal _impactnormal _physmat _hitactor) (`GameplayStatics.BreakHitResult` (`self.GetHitResultUnderCursorForObjects` (`GameplayStatics.GetPlayerController` 0) (`|MakeArray` "ObjectTypeQuery2" :!type "EObjectTypeQuery Enum") true)))
  ;[1 1 1] Select Target
  (if (`self.ActorHasTag` _hitactor "Enemy")
    (set `self.TargetActor` _hitactor :!label _label)
    (switch `/Game/Blueprints/Heroes/E_ActionTypes` (`self.ActionTypes`)
      (:`NewEnumerator0`
        (bind _returnvalue (`self.IsTargetFrontRow`))
        (if _returnvalue
          (`self.Pound`)
          (`/Game/Blueprints/BP_GameMode.CheckHeroActionsComplete` (`self.GameMode`))
          (else
            (`KismetSystemLibrary.PrintString` "Target is not in front row"))))
      (:`NewEnumerator1`
        (`self.ThrowShade`)
        (`/Game/Blueprints/BP_GameMode.CheckHeroActionsComplete` (`self.GameMode`)))
      (:`NewEnumerator2`
        (`self.Seduce`)
        (set `/Game/Blueprints/BP_GameMode.ActiveHero` null (`self.GameMode`)) ; Set Active Hero to null
        (`/Game/Blueprints/BP_GameMode.CheckHeroActionsComplete` (`self.GameMode`)))
      (:`NewEnumerator6`
        (bind _returnvalue_2 (`GameplayStatics.GetActorOfClass` "/Game/Blueprints/Drama/BP_DramaBase.BP_DramaBase_C"))
        (message `/Game/Blueprints/Drama/BPI_DramaAbility.EndDrama` _returnvalue_2 (`self.TargetActor`))))
    (elif (`self.ActorHasTag` _hitactor "Hero")
      (goto _label))))

(fn `DecrementActionPoint`
  (bind _activehero (`/Game/Blueprints/BP_GameMode.ActiveHero` (`self.GameMode`)))
  (`/Engine/EditorBlueprintResources/StandardMacros.DecrementInt` (`/Game/Blueprints/Heroes/BP_HeroBase.ActionPoints` _activehero)
    (:`  `
      (`/Game/Blueprints/Heroes/BP_HeroBase.SetActionPointsWidget` _activehero))))

(fn `Defend`
  (`/Game/Blueprints/Heroes/BP_HeroBase.IncreaseShield` (`/Game/Blueprints/BP_GameMode.ActiveHero` (`self.GameMode`)))
  (`KismetSystemLibrary.PrintString` "Defend")
  (set `self.SelectingTarget` false)
  (`self.DecrementActionPoint`)
  (set `/Game/Blueprints/BP_GameMode.ActiveHero` null (`self.GameMode`)))

(fn `IsFrontRowOccupied`
  (returns (ReturnValue :type Boolean))
  (for _array_element (`/Game/Blueprints/BP_GameState.EnemyPositions` (`/Game/Blueprints/BP_GameMode.As BP Game State` (`self.GameMode`)))
    (bind _returnvalue (== (`.Row_17_E8C0F1744089718EC0A17D945359F830` (break `/Game/Blueprints/Battlefield/F_EnemyPosition` _array_element)) (`self.FrontRow`)))
    (if _returnvalue
      (return _returnvalue))))

(fn `IsTargetFrontRow`
  (returns (ReturnValue :type Boolean))
  (for _array_element (`/Game/Blueprints/BP_GameState.EnemyPositions` (`/Game/Blueprints/BP_GameMode.As BP Game State` (`self.GameMode`)))
    (bind (_enemy _type _column _row) (break `/Game/Blueprints/Battlefield/F_EnemyPosition` _array_element))
    (if (== _enemy (`self.TargetActor`))
      (return (== _row (`self.FrontRow`))))))

(fn `MoveActiveHeroBackstage`
  (params (ActiveHero :type "/Game/Blueprints/Heroes/BP_HeroBase Object Reference"))
  (bind _backstage (`/Game/Blueprints/BP_GameMode.Backstage` (`self.GameMode`)))
  (set `/Game/Blueprints/Heroes/BP_HeroBase.StageLocation` _backstage ActiveHero)
  (`self.K2_SetActorLocation` ActiveHero (`self.K2_GetActorLocation` _backstage) false false)
  (bind _returnvalue (`|CreateWidget` "/Game/UI/HeroBackstageWidgets/WBP_Hero.WBP_Hero_C" null (`/Game/Blueprints/Heroes/BP_HeroBase.HeroStats` ActiveHero)))
  (`/Game/UI/WBP_HeroHUD.AddHeroBackstage` (`/Game/Blueprints/BP_GameMode.HUD` (`self.GameMode`)) _returnvalue (`/Game/Blueprints/Heroes/BP_HeroBase.Pounded` ActiveHero)))

(fn `Pound`
  (bind _activehero (`/Game/Blueprints/BP_GameMode.ActiveHero` (`self.GameMode`)))
  (bind (_totaldamage _pounddamage) (`/Game/Blueprints/Heroes/BP_HeroBase.CalculatePoundDamage` _activehero))
  (bind _asbp_enemy_base (cast `/Game/Blueprints/Enemies/BP_EnemyBase` (`self.TargetActor`)))
  (message `/Game/Blueprints/ActorComponents/BPI_DamageHandling.DamageHandling` (`/Game/Blueprints/Enemies/BP_EnemyBase.BP_Health` _asbp_enemy_base) _pounddamage _activehero "NewEnumerator0")
  (set `self.SelectingTarget` false)
  (`self.DecrementActionPoint`)
  (set `/Game/Blueprints/BP_GameMode.ActiveHero` null (`self.GameMode`)) ; Set Active Hero to null
)

(fn `PullOut`
  (bind _gamemode (`self.GameMode`))
  (bind _activehero (`/Game/Blueprints/BP_GameMode.ActiveHero` (`self.GameMode`)))
  (bind _asbp_hero_base (cast `/Game/Blueprints/Heroes/BP_HeroBase` (`self.TargetActor`)))
  (`/Game/Blueprints/Heroes/BP_HeroBase.PulloutActionPointHandling` _asbp_hero_base)
  (`/Game/Blueprints/Heroes/BP_HeroBase.MoveHeroOnstage` _asbp_hero_base (`/Game/Blueprints/Heroes/BP_HeroBase.StageLocation` _activehero))
  (`/Engine/EditorBlueprintResources/StandardMacros.DecrementInt` (`/Game/Blueprints/Heroes/BP_HeroBase.ActionPoints` _activehero)
    (:`  `
      (`self.MoveActiveHeroBackstage` _activehero)
      (`/Game/Blueprints/BP_GameMode.CheckHeroActionsComplete` _gamemode)
      (set `/Game/Blueprints/BP_GameMode.ActiveHero` null _gamemode)
      (set `self.SelectingHero` false)
      (set `self.TargetActor` null)
      (`KismetSystemLibrary.PrintString` "Pull Out" true true (struct :`R` 0.444579 :`B` 0.644097 :`A` 1.0)))))

(fn `RemoveSeducedEnemy`
  (params (EnemyTarget :type "Object Object Reference"))
  (bind _enemypositions (`/Game/Blueprints/BP_GameState.EnemyPositions` (`/Game/Blueprints/BP_GameMode.As BP Game State` (`self.GameMode`))))
  (for _array_element _enemypositions
    (if (== (`.Enemy_8_0A2295EE40072C1942B114ADBC16CCE4` (break `/Game/Blueprints/Battlefield/F_EnemyPosition` _array_element)) EnemyTarget)
      (`KismetArrayLibrary.Array_RemoveItem` _enemypositions _array_element))))

(fn `Seduce`
  (locals (EnemyTarget :type "/Game/Blueprints/Enemies/BP_EnemyBase Object Reference") (SeduceValue :type Integer :default 0))
  (bind _enemytarget (`local.EnemyTarget`))
  (bind _gamemode (`self.GameMode`))
  (bind _activehero (`/Game/Blueprints/BP_GameMode.ActiveHero` _gamemode))
  (bind _asbp_enemy_base (cast `/Game/Blueprints/Enemies/BP_EnemyBase` (`self.TargetActor`))
    (:`then`
      (if (`/Game/Blueprints/Enemies/BP_EnemyBase.Heartless` _asbp_enemy_base)
        (`KismetSystemLibrary.PrintString` "Not a valid Seduce Target" :!label _label)
        (else
          (set `local.EnemyTarget` _asbp_enemy_base)
          (set `local.SeduceValue` (+ (`.Passion_5_34B7CC1B49BD8269316506884D42E651` (break `/Game/Blueprints/Heroes/F_HeroStats` (`/Game/Blueprints/Heroes/BP_HeroBase.HeroStats` (`/Game/Blueprints/BP_GameMode.ActiveHero` (`self.GameMode`))))) 1))
          (`|ExecutionSequence`
            (:`then_0`
              (`/Engine/EditorBlueprintResources/StandardMacros.Do N` (`local.SeduceValue`) :!label _label_2
                (:`Exit`
                  (if (not (`/Game/Blueprints/Enemies/BP_EnemyBase.Seduced` (`local.EnemyTarget`)))
                    (if (>= (`KismetMathLibrary.RandomIntegerInRange` 1 6) (`/Game/Blueprints/Enemies/BP_EnemyBase.Chastity` (`local.EnemyTarget`)))
                      (set `/Game/Blueprints/Enemies/BP_EnemyBase.Seduced` true (`local.EnemyTarget`))
                      (`self.K2_SetActorLocation` (`local.EnemyTarget`) (`SceneComponent.K2_GetComponentLocation` (`/Game/Blueprints/Heroes/BP_HeroBase.SeducedLocation` _activehero)) false false)
                      (set `/Game/Blueprints/Heroes/BP_HeroBase.SeducedEnemy` (`local.EnemyTarget`) _activehero)
                      (set `/Game/Blueprints/Heroes/BP_HeroBase.HasSeducedEnemy` true _activehero)
                      (`self.RemoveSeducedEnemy` (`local.EnemyTarget`))
                      (`/Game/Blueprints/BP_GameMode.CheckEnemyPresence` _gamemode)
                      (`/Game/Blueprints/BP_GameMode.SetEnemyIntentions` _gamemode)
                      (`self.DecrementActionPoint`)
                      (set `self.SelectingTarget` false)
                      (else
                        (`KismetSystemLibrary.PrintString` "Seduce Failed")
                        (goto _label_2)))))))
            (:`then_1`
              (set `/Game/Blueprints/Enemies/BP_EnemyBase.Chastity` (- (`/Game/Blueprints/Enemies/BP_EnemyBase.Chastity` _enemytarget) (`local.SeduceValue`)) _enemytarget)
              (if (not (`/Game/Blueprints/Heroes/BP_HeroBase.HasSeducedEnemy` (`/Game/Blueprints/BP_GameMode.ActiveHero` (`self.GameMode`))))
                (`self.DecrementActionPoint`)
                (set `self.SelectingTarget` false)))))))
    (:`CastFailed`
      (goto _label))))

(fn `SetFrontRow`
  (locals (`ValidTargets (L)` :type "Array of Actor Object Reference") (`Enemies (L)` :type "Array of /Game/Blueprints/Battlefield/F_EnemyPosition Structure") (`Row (L)` :type Integer))
  (bind _output_get (set `local.Enemies (L)` (`/Game/Blueprints/BP_GameState.EnemyPositions` (`/Game/Blueprints/BP_GameMode.As BP Game State` (`self.GameMode`)))))
  (for _array_element _output_get
    (bind (_enemy _type _column _row) (break `/Game/Blueprints/Battlefield/F_EnemyPosition` _array_element))
    (if (== _row (`local.Row (L)`))
      (`KismetArrayLibrary.Array_Add` (`local.ValidTargets (L)`) _enemy)))
  (if (== (`KismetArrayLibrary.Array_Length` (`local.ValidTargets (L)`)) 0)
    (`/Engine/EditorBlueprintResources/StandardMacros.IncrementInt` (`local.Row (L)`)
      (:`  `
        (for _array_element_2 (`local.Enemies (L)`)
          (bind (_enemy_2 _type_2 _column_2 _row_2) (break `/Game/Blueprints/Battlefield/F_EnemyPosition` _array_element_2))
          (if (== _row_2 (`local.Row (L)`))
            (`KismetArrayLibrary.Array_Add` (`local.ValidTargets (L)`) _enemy_2)))
        (if (== (`KismetArrayLibrary.Array_Length` (`local.ValidTargets (L)`)) 0)
          (bind _result (`/Engine/EditorBlueprintResources/StandardMacros.IncrementInt` (`local.Row (L)`))
            (:`  `
              (set `self.FrontRow` _result)))
          (else
            (set `self.FrontRow` (`local.Row (L)`))))))
    (else
      (set `self.FrontRow` (`local.Row (L)`)))))

(fn `ThrowShade`
  (bind _activehero (`/Game/Blueprints/BP_GameMode.ActiveHero` (`self.GameMode`)))
  (`KismetSystemLibrary.PrintString` "Throw Shade")
  (bind _totaldamage (`/Game/Blueprints/Heroes/BP_HeroBase.CalculateThrowShadeDamage` _activehero))
  (bind _asbp_enemy_base (cast `/Game/Blueprints/Enemies/BP_EnemyBase` (`self.TargetActor`)))
  (message `/Game/Blueprints/ActorComponents/BPI_DamageHandling.DamageHandling` (`/Game/Blueprints/Enemies/BP_EnemyBase.BP_Health` _asbp_enemy_base) (`KismetMathLibrary.FTrunc` _totaldamage) _activehero "NewEnumerator1")
  (set `self.SelectingTarget` false)
  (`self.DecrementActionPoint`)
  (set `/Game/Blueprints/BP_GameMode.ActiveHero` null (`self.GameMode`)))

(fn `UserConstructionScript`)

(fn `WasActiveHeroClicked`
  (returns (ReturnValue :type Boolean))
  (return (== (`.HitActor` (`GameplayStatics.BreakHitResult` (`self.GetHitResultUnderCursorForObjects` (`GameplayStatics.GetPlayerController` 0) (`|MakeArray` "ObjectTypeQuery1" "ObjectTypeQuery3" "ObjectTypeQuery2" :!type "EObjectTypeQuery Enum") true))) (`/Game/Blueprints/BP_GameMode.ActiveHero` (`self.GameMode`)))))