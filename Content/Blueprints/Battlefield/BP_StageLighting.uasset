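; BP_StageLighting controls the house lights for a battlefield stage through a directional light that starts at a low intensity.
; HouseLightsUp plays a timeline whose alpha lerps the light intensity from LowLights to BrightLights.
; HouseLightsDown reverses the same timeline to fade the light back down.
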(event `self.ReceiveBeginPlay`
  (`LightComponent.SetIntensity` (`self.DirectionalLight`) (`self.LowLights`)))

(event `HouseLightsUp`
  (bind (_direction _lightsalpha) (`Timeline|LerpLightIntensity` :!via `PlayFromStart` :!label _label)
    (:`Update`
      (`LightComponent.SetIntensity` (`self.DirectionalLight`) (`KismetMathLibrary.Lerp` (`self.LowLights`) (`self.BrightLights`) _lightsalpha)))))

(event `HouseLightsDown`
  (goto _label :!via `Reverse`))

(fn `UserConstructionScript`)