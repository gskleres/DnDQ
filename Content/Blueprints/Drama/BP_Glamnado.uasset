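; Glamnado drama ability actor: a hero targets an enemy outside the back row to push that enemy's row back one stage row.
; StartDrama records the caster; EndDrama finds the target's row, collects enemies with free space behind, and moves them to matching BP_EnemyPosition actors, updating GameState positions.
; It then refreshes enemy intentions, spends an action point and shared alcohol, ends targeting, and destroys itself.
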(event `/Game/Blueprints/Drama/BPI_DramaAbility.StartDrama`
  (set `self.CastingActor` (`/Game/Blueprints/BP_GameMode.ActiveHero` (`self.As BP Game Mode`)))
  (for _array_element (`self.AffectedEnemies`)
    (`KismetSystemLibrary.PrintString` (`KismetSystemLibrary.GetDisplayName` _array_element))))

(event `/Game/Blueprints/Drama/BPI_DramaAbility.EndDrama`
  (params (TargetActor :type "Actor Object Reference"))
  (bind _asbp_enemy_base (cast `/Game/Blueprints/Enemies/BP_EnemyBase` TargetActor)
    (:`then`
      (set `self.TargetEnemy` _asbp_enemy_base)
      (`self.GetEnemyRow`)
      (if (== (`self.TargetRow`) (`self.BackRow`))
        (`KismetSystemLibrary.PrintString` "Cannot Target Back Row")
        (else
          (`self.SetAffectedEnemies`)
          (`self.MoveAffectedEnemies`)
          (`KismetSystemLibrary.PrintString` "Complete")
          (`/Game/Blueprints/BP_GameMode.SetEnemyIntentions` (`self.As BP Game Mode`))
          (`self.CompleteGlamnado`))))
    (:`CastFailed`
      (`KismetSystemLibrary.PrintString` "Not a valid target"))))

(fn `CompleteGlamnado`
  (bind _castingactor (`self.CastingActor`))
  (bind _as_bp_game_mode (`self.As BP Game Mode`))
  (`/Engine/EditorBlueprintResources/StandardMacros.DecrementInt` (`/Game/Blueprints/Heroes/BP_HeroBase.ActionPoints` _castingactor)
    (:`  `
      (`/Game/Blueprints/Heroes/BP_HeroBase.SetActionPointsWidget` _castingactor)
      (`/Engine/EditorBlueprintResources/StandardMacros.DecrementInt` (`/Game/Blueprints/BP_GameMode.AlcoholPool` _as_bp_game_mode)
        (:`  `
          (set `/Game/Blueprints/BP_GameMode.ActiveHero` null _as_bp_game_mode) ; Set Active Hero to null
          (`/Game/Blueprints/BP_GameMode.CheckHeroActionsComplete` _as_bp_game_mode)
          (set `/Game/Blueprints/BP_PlayerController.SelectingTarget` false (`self.As BP Player Controller`))
          (`self.K2_DestroyActor`))))))

(fn `GetEnemyRow`
  (for _array_element (`/Game/Blueprints/BP_GameState.EnemyPositions` (`/Game/Blueprints/BP_GameMode.As BP Game State` (`self.As BP Game Mode`)))
    (bind ((`Enemy_8_0A2295EE40072C1942B114ADBC16CCE4` _enemy) (`Row_17_E8C0F1744089718EC0A17D945359F830` _row)) (break `/Game/Blueprints/Battlefield/F_EnemyPosition` _array_element))
    (if (== _enemy (`self.TargetEnemy`))
      (bind _output_get (set `self.TargetRow` _row))))
  (return))

(fn `MoveAffectedEnemies`
  (bind _enemypositions (`/Game/Blueprints/BP_GameState.EnemyPositions` (`/Game/Blueprints/BP_GameMode.As BP Game State` (`self.As BP Game Mode`))))
  (for _array_element (`self.AffectedEnemies`)
    (bind _asbp_enemy_position (cast `/Game/Blueprints/Battlefield/BP_EnemyPosition` (`/Game/Blueprints/Enemies/BP_EnemyBase.Position` _array_element)))
    (bind _outactors (`GameplayStatics.GetAllActorsOfClass` "/Game/Blueprints/Battlefield/BP_EnemyPosition.BP_EnemyPosition_C"))
    (for _array_element_2 _outactors
      (bind _stage_column (`/Game/Blueprints/Battlefield/BP_EnemyPosition.Stage_Column` _array_element_2))
      (bind _returnvalue (+ (`/Game/Blueprints/Battlefield/BP_EnemyPosition.Stage_Row` _asbp_enemy_position) 1))
      (if (and (== _stage_column (`/Game/Blueprints/Battlefield/BP_EnemyPosition.Stage_Column` _asbp_enemy_position)) (== (`/Game/Blueprints/Battlefield/BP_EnemyPosition.Stage_Row` _array_element_2) _returnvalue))
        (`self.K2_SetActorLocation` _array_element (`self.K2_GetActorLocation` _array_element_2) false false)
        (set `/Game/Blueprints/Enemies/BP_EnemyBase.Position` _array_element_2 _array_element)
        (for (_array_element_3 _array_index) _enemypositions
          (bind (_enemy _type) (break `/Game/Blueprints/Battlefield/F_EnemyPosition` _array_element_3))
          (if (== _enemy _array_element)
            (`KismetArrayLibrary.Array_Set` _enemypositions _array_index (make `/Game/Blueprints/Battlefield/F_EnemyPosition` _enemy _type _stage_column _returnvalue))))))))

(fn `SetAffectedEnemies`
  (for _array_element (`/Game/Blueprints/BP_GameState.EnemyPositions` (`/Game/Blueprints/BP_GameMode.As BP Game State` (`self.As BP Game Mode`)))
    (bind (_enemy _type _column _row) (break `/Game/Blueprints/Battlefield/F_EnemyPosition` _array_element))
    (if (== _row (`self.TargetRow`))
      (for _array_element_2 (`/Game/Blueprints/BP_GameState.EnemyPositions` (`/Game/Blueprints/BP_GameMode.As BP Game State` (`self.As BP Game Mode`)))
        (bind (_enemy_2 _type_2 _column_2 _row_2) (break `/Game/Blueprints/Battlefield/F_EnemyPosition` _array_element_2))
        (if (and (== _column_2 _column) (== _row_2 (+ _row 1)))
          (set `self.PositionBlocked` true)))
      (if (`self.PositionBlocked`)
        (set `self.PositionBlocked` false)
        (else
          (bind _asbp_enemy_base (cast `/Game/Blueprints/Enemies/BP_EnemyBase` _enemy))
          (`KismetArrayLibrary.Array_Add` (`self.AffectedEnemies`) _asbp_enemy_base))))))

(fn `UserConstructionScript`
  (`parent.UserConstructionScript`))