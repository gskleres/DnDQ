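; Hot Sauce drama ability that lets each onstage hero attempt to seduce a chosen non-Heartless enemy.
; StartDrama gathers heroes and targets; each EndDrama selection uses the next hero until either list empties.
; AttemptSeduce loops d6 rolls (Passion+1) against Chastity, moves seduced enemies to the hero, and lowers Chastity regardless.
; Completion spends the caster's action point and one AlcoholPool, then destroys the actor.
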(event `/Game/Blueprints/Drama/BPI_DramaAbility.StartDrama`
  (set `self.CastingActor` (`/Game/Blueprints/BP_GameMode.ActiveHero` (`self.As BP Game Mode`)))
  (`KismetArrayLibrary.Array_Clear` (`self.Heroes`))
  (`KismetArrayLibrary.Array_Clear` (`self.HotSauceTargets`))
  (`self.SetPossibleTargets`)
  (`self.SetHeroesOnstage`))

(event `/Game/Blueprints/Drama/BPI_DramaAbility.EndDrama`
  (params (TargetActor :type "Actor Object Reference"))
  (bind _asbp_enemy_base (cast `/Game/Blueprints/Enemies/BP_EnemyBase` TargetActor))
  (for (_array_element _array_index) (`self.Heroes`)
    (if (== _array_index 0)
      (if (not (`/Game/Blueprints/Enemies/BP_EnemyBase.Heartless` _asbp_enemy_base))
        (`self.AttemptSeduce` _asbp_enemy_base _array_element)
        (`KismetArrayLibrary.Array_RemoveItem` (`self.Heroes`) _array_element)
        (if (> (`KismetArrayLibrary.Array_Length` (`self.HotSauceTargets`)) 0)
          (if (> (`KismetArrayLibrary.Array_Length` (`self.Heroes`)) 0)
            (`KismetSystemLibrary.PrintString` "Select Again")
            (else
              (`self.HotSauceComplete`)))
          (else
            (`self.HotSauceComplete`)))
        (else
          (`KismetSystemLibrary.PrintString` "Not a valid Seduce Target"))))))

(fn `AttemptSeduce`
  (params (Enemy :type "/Game/Blueprints/Enemies/BP_EnemyBase Object Reference") (Hero :type "/Game/Blueprints/Heroes/BP_HeroBase Object Reference"))
  (locals (EnemyTarget :type "/Game/Blueprints/Enemies/BP_EnemyBase Object Reference") (SeduceValue :type Integer))
  (bind _enemytarget (`local.EnemyTarget`))
  (bind _enemytarget_2 (`local.EnemyTarget`))
  (bind _as_bp_game_mode (`self.As BP Game Mode`))
  (bind _hero (`local.Hero`))
  (set `local.EnemyTarget` Enemy)
  (set `local.SeduceValue` (+ (`.Passion_5_34B7CC1B49BD8269316506884D42E651` (break `/Game/Blueprints/Heroes/F_HeroStats` (`/Game/Blueprints/Heroes/BP_HeroBase.HeroStats` Hero))) 1))
  (`|ExecutionSequence`
    (:`then_0`
      (`/Engine/EditorBlueprintResources/StandardMacros.Do N` (`local.SeduceValue`) :!label _label
        (:`Exit`
          (if (not (`/Game/Blueprints/Enemies/BP_EnemyBase.Seduced` (`local.EnemyTarget`)))
            (if (>= (`KismetMathLibrary.RandomIntegerInRange` 1 6) (`/Game/Blueprints/Enemies/BP_EnemyBase.Chastity` (`local.EnemyTarget`)))
              (set `/Game/Blueprints/Enemies/BP_EnemyBase.Seduced` true (`local.EnemyTarget`))
              (`self.K2_SetActorLocation` (`local.EnemyTarget`) (`SceneComponent.K2_GetComponentLocation` (`/Game/Blueprints/Heroes/BP_HeroBase.SeducedLocation` _hero)) false false)
              (set `/Game/Blueprints/Heroes/BP_HeroBase.SeducedEnemy` (`local.EnemyTarget`) _hero)
              (set `/Game/Blueprints/Heroes/BP_HeroBase.HasSeducedEnemy` true _hero)
              (`KismetArrayLibrary.Array_RemoveItem` (`self.HotSauceTargets`) _enemytarget)
              (`self.RemoveEnemy` _enemytarget)
              (`/Game/Blueprints/BP_GameMode.CheckEnemyPresence` _as_bp_game_mode)
              (`/Game/Blueprints/BP_GameMode.SetEnemyIntentions` _as_bp_game_mode)
              (else
                (`KismetSystemLibrary.PrintString` "Seduce Failed")
                (goto _label)))))))
    (:`then_1`
      (set `/Game/Blueprints/Enemies/BP_EnemyBase.Chastity` (- (`/Game/Blueprints/Enemies/BP_EnemyBase.Chastity` _enemytarget_2) (`local.SeduceValue`)) _enemytarget_2)
      (if (not (`/Game/Blueprints/Heroes/BP_HeroBase.HasSeducedEnemy` (`local.Hero`)))
        (`KismetSystemLibrary.PrintString` "Seduce Missed")))))

(fn `HotSauceComplete`
  (bind _as_bp_game_mode (`self.As BP Game Mode`))
  (bind _castingactor (`self.CastingActor`))
  (`/Engine/EditorBlueprintResources/StandardMacros.DecrementInt` (`/Game/Blueprints/Heroes/BP_HeroBase.ActionPoints` _castingactor)
    (:`  `
      (`/Game/Blueprints/Heroes/BP_HeroBase.SetActionPointsWidget` _castingactor)
      (`/Engine/EditorBlueprintResources/StandardMacros.DecrementInt` (`/Game/Blueprints/BP_GameMode.AlcoholPool` _as_bp_game_mode)
        (:`  `
          (set `/Game/Blueprints/BP_GameMode.ActiveHero` null _as_bp_game_mode) ; Set Active Hero to null
          (`/Game/Blueprints/BP_GameMode.CheckHeroActionsComplete` _as_bp_game_mode)
          (set `/Game/Blueprints/BP_PlayerController.SelectingTarget` false (`self.As BP Player Controller`))
          (`KismetSystemLibrary.PrintString` "Hot Sauce Complete")
          (`self.K2_DestroyActor`))))))

(fn `IsHeroOnstage`
  (params (Hero :type "/Game/Blueprints/Heroes/BP_HeroBase Object Reference"))
  (returns (Onstage :type Boolean))
  (bind _returnvalue (`GameplayStatics.GetObjectClass` (`/Game/Blueprints/Heroes/BP_HeroBase.StageLocation` Hero)))
  (return (or (== _returnvalue "/Game/Blueprints/Battlefield/StagePositions/BP_Spotlight.BP_Spotlight_C") (== _returnvalue "/Game/Blueprints/Battlefield/StagePositions/BP_StageLeft.BP_StageLeft_C") (== _returnvalue "/Game/Blueprints/Battlefield/StagePositions/BP_StageRight.BP_StageRight_C"))))

(fn `RemoveEnemy`
  (params (Enemy :type "/Game/Blueprints/Enemies/BP_EnemyBase Object Reference"))
  (bind _enemypositions (`/Game/Blueprints/BP_GameState.EnemyPositions` (`/Game/Blueprints/BP_GameMode.As BP Game State` (`self.As BP Game Mode`))))
  (for _array_element _enemypositions
    (if (== (`.Enemy_8_0A2295EE40072C1942B114ADBC16CCE4` (break `/Game/Blueprints/Battlefield/F_EnemyPosition` _array_element)) Enemy)
      (`KismetArrayLibrary.Array_RemoveItem` _enemypositions _array_element))))

(fn `SetHeroesOnstage`
  (bind _outactors (`GameplayStatics.GetAllActorsOfClass` "/Game/Blueprints/Heroes/BP_HeroBase.BP_HeroBase_C"))
  (for _array_element _outactors
    (if (`self.IsHeroOnstage` _array_element)
      (`KismetArrayLibrary.Array_Add` (`self.Heroes`) _array_element))))

(fn `SetPossibleTargets`
  (locals (NewLocalVar_0 :type "Array of /Game/Blueprints/Enemies/BP_EnemyBase Object Reference"))
  (bind _outactors (`GameplayStatics.GetAllActorsOfClass` "/Game/Blueprints/Enemies/BP_EnemyBase.BP_EnemyBase_C"))
  (for _array_element _outactors
    (if (not (`/Game/Blueprints/Enemies/BP_EnemyBase.Heartless` _array_element))
      (`KismetArrayLibrary.Array_Add` (`local.NewLocalVar_0`) _array_element)))
  (bind _output_get (set `self.HotSauceTargets` (`local.NewLocalVar_0`)))
  (`KismetSystemLibrary.PrintString` (`KismetStringLibrary.Concat_StrStr` "Possible Targets: " (`KismetStringLibrary.Conv_IntToString` (`KismetArrayLibrary.Array_Length` _output_get)))))

(fn `UserConstructionScript`
  (`parent.UserConstructionScript`))