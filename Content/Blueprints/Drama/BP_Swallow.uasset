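; BP_Swallow is a hero Drama action that deals mental damage to a chosen front-row enemy, chaining while targets die.
; StartDrama caches the active hero and row-zero enemies; EndDrama damages the selected one.
; If it stays valid, the action completes; otherwise it leaves the list and selection continues until none remain.
; Completion spends an action point and alcohol, releases the hero and destroys the actor; having no targets skips the cost.
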(event `/Game/Blueprints/Drama/BPI_DramaAbility.StartDrama`
  (set `self.CastingActor` (`/Game/Blueprints/BP_GameMode.ActiveHero` (`self.As BP Game Mode`)))
  (for _array_element (`/Game/Blueprints/BP_GameState.EnemyPositions` (`/Game/Blueprints/BP_GameMode.As BP Game State` (`self.As BP Game Mode`)))
    (bind ((`Enemy_8_0A2295EE40072C1942B114ADBC16CCE4` _enemy) (`Row_17_E8C0F1744089718EC0A17D945359F830` _row)) (break `/Game/Blueprints/Battlefield/F_EnemyPosition` _array_element))
    (if (== _row 0)
      (bind _asbp_enemy_base (cast `/Game/Blueprints/Enemies/BP_EnemyBase` _enemy))
      (`KismetArrayLibrary.Array_Add` (`self.PossibleTargets`) _asbp_enemy_base)))
  (`self.CheckStartingTargets`))

(event `/Game/Blueprints/Drama/BPI_DramaAbility.EndDrama`
  (params (TargetActor :type "Actor Object Reference"))
  (if (> (`KismetArrayLibrary.Array_Length` (`self.PossibleTargets`)) 0)
    (bind _asbp_enemy_base (cast `/Game/Blueprints/Enemies/BP_EnemyBase` TargetActor)
      (:`then`
        (bind _output_get (set `self.EnemyTarget` _asbp_enemy_base))
        (for _array_element (`self.PossibleTargets`)
          (if (== _array_element _output_get)
            (`GameplayStatics.ApplyDamage` _array_element (`self.SwallowDamage`) null (`self.CastingActor`) "/Game/Blueprints/DamageTypes/BP_MentalDamage.BP_MentalDamage_C")
            (`/Engine/EditorBlueprintResources/StandardMacros.IsValid` _array_element
              (:`Is Valid`
                (`KismetSystemLibrary.PrintString` "Enemy Didn't Die")
                (`self.SwallowComplete`))
              (:`Is Not Valid`
                (`KismetArrayLibrary.Array_RemoveItem` (`self.PossibleTargets`) (`self.EnemyTarget`))))
            (else
              (`KismetSystemLibrary.PrintString` "Enemy not in front row"))))
        (`self.CheckPossibleTargets`))
      (:`CastFailed`
        (`KismetSystemLibrary.PrintString` "Not a Valid Target")))
    (else
      (`self.NoTargets`))))

(fn `CheckPossibleTargets`
  (bind _returnvalue (`KismetArrayLibrary.Array_Length` (`self.PossibleTargets`)))
  (if (== _returnvalue 0)
    (`self.SwallowComplete`)
    (else
      (`KismetSystemLibrary.PrintString` (`KismetStringLibrary.Conv_IntToString` _returnvalue)))))

(fn `CheckStartingTargets`
  (bind _returnvalue (`KismetArrayLibrary.Array_Length` (`self.PossibleTargets`)))
  (if (== _returnvalue 0)
    (`KismetSystemLibrary.PrintString` "No Targets")
    (else
      (`KismetSystemLibrary.PrintString` (`KismetStringLibrary.Conv_IntToString` _returnvalue)))))

(fn `NoTargets`
  (bind _as_bp_game_mode (`self.As BP Game Mode`))
  (set `/Game/Blueprints/BP_GameMode.ActiveHero` null _as_bp_game_mode) ; Set Active Hero to null
  (`/Game/Blueprints/BP_GameMode.CheckHeroActionsComplete` _as_bp_game_mode)
  (set `/Game/Blueprints/BP_PlayerController.SelectingTarget` false (`self.As BP Player Controller`))
  (`KismetSystemLibrary.PrintString` "No Valid Swallow Targets")
  (`self.K2_DestroyActor`))

(fn `SwallowComplete`
  (bind _as_bp_game_mode (`self.As BP Game Mode`))
  (bind _castingactor (`self.CastingActor`))
  (`/Engine/EditorBlueprintResources/StandardMacros.DecrementInt` (`/Game/Blueprints/Heroes/BP_HeroBase.ActionPoints` _castingactor)
    (:`  `
      (`/Game/Blueprints/Heroes/BP_HeroBase.SetActionPointsWidget` _castingactor)
      (`/Engine/EditorBlueprintResources/StandardMacros.DecrementInt` (`/Game/Blueprints/BP_GameMode.AlcoholPool` _as_bp_game_mode)
        (:`  `
          (set `/Game/Blueprints/BP_GameMode.ActiveHero` null _as_bp_game_mode) ; Set Active Hero to null
          (`/Game/Blueprints/BP_GameMode.CheckHeroActionsComplete` _as_bp_game_mode)
          (set `/Game/Blueprints/BP_PlayerController.SelectingTarget` false (`self.As BP Player Controller`))
          (`KismetSystemLibrary.PrintString` "Swallow Complete")
          (`self.K2_DestroyActor`))))))

(fn `UserConstructionScript`
  (`parent.UserConstructionScript`))