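; BP_TwinFang is a hero "Drama" ability that damages two enemies chosen one after another.
; StartDrama records the active hero as caster, and each EndDrama call accepts only BP_EnemyBase targets, storing the first and striking both through BPHealth once the second arrives.
; TwinFangComplete then spends an action point and AlcoholPool, clears the active hero, checks whether hero actions are complete, ends target selection and destroys the actor.
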(event `/Game/Blueprints/Drama/BPI_DramaAbility.StartDrama`
  (set `self.CastingActor` (`/Game/Blueprints/BP_GameMode.ActiveHero` (`self.As BP Game Mode`))))

(event `/Game/Blueprints/Drama/BPI_DramaAbility.EndDrama`
  (params (TargetActor :type "Actor Object Reference"))
  (bind _asbp_enemy_base (cast `/Game/Blueprints/Enemies/BP_EnemyBase` TargetActor)
    (:`then`
      (set `self.EnemyTarget` _asbp_enemy_base)
      (if (== (`self.Target1`) null)
        (set `self.Target1` (`self.EnemyTarget`))
        (else
          (set `self.Target2` (`self.EnemyTarget`))
          (message `/Game/Blueprints/ActorComponents/BPI_DamageHandling.DamageHandling` (`/Game/Blueprints/Enemies/BP_EnemyBase.BP_Health` (`self.Target1`)) (`self.DamageAmount`) (`self.CastingActor`) "NewEnumerator5")
          (`KismetSystemLibrary.Delay` 0.1)
          (message `/Game/Blueprints/ActorComponents/BPI_DamageHandling.DamageHandling` (`/Game/Blueprints/Enemies/BP_EnemyBase.BP_Health` (`self.Target2`)) (`self.DamageAmount`) (`self.CastingActor`) "NewEnumerator5")
          (`self.TwinFangComplete`))))
    (:`CastFailed`
      (`KismetSystemLibrary.PrintString` "Not a Valid Target"))))

(fn `SelectTargetOne`
  (bind _output_get (set `self.Target1` (`self.EnemyTarget`)))
  (`KismetSystemLibrary.PrintString` (`KismetStringLibrary.Concat_StrStr` "Target 1: " (`KismetSystemLibrary.GetDisplayName` _output_get))))

(fn `TwinFangComplete`
  (bind _castingactor (`self.CastingActor`))
  (bind _as_bp_game_mode (`self.As BP Game Mode`))
  (`/Engine/EditorBlueprintResources/StandardMacros.DecrementInt` (`/Game/Blueprints/Heroes/BP_HeroBase.ActionPoints` _castingactor)
    (:`  `
      (`/Game/Blueprints/Heroes/BP_HeroBase.SetActionPointsWidget` _castingactor)
      (`/Engine/EditorBlueprintResources/StandardMacros.DecrementInt` (`/Game/Blueprints/BP_GameMode.AlcoholPool` _as_bp_game_mode)
        (:`  `
          (set `/Game/Blueprints/BP_GameMode.ActiveHero` null _as_bp_game_mode) ; Set Active Hero to null
          (`/Game/Blueprints/BP_GameMode.CheckHeroActionsComplete` _as_bp_game_mode)
          (set `/Game/Blueprints/BP_PlayerController.SelectingTarget` false (`self.As BP Player Controller`))
          (`self.K2_DestroyActor`))))))

(fn `UserConstructionScript`
  (`parent.UserConstructionScript`))