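; BP_Zinger is a targeted Drama action that shocks and stuns an enemy.
; EndDrama accepts only BP_EnemyBase targets, applies shock damage, then sets the stun state and duration if the enemy is still valid.
; It then refreshes enemy intentions, spends one AlcoholPool point and one of the active hero's action points, clears hero and target selection, and destroys itself.
; StartDrama is empty.
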(event `/Game/Blueprints/Drama/BPI_DramaAbility.StartDrama`)

(event `/Game/Blueprints/Drama/BPI_DramaAbility.EndDrama`
  (params (TargetActor :type "Actor Object Reference"))
  (bind _as_bp_game_mode (`self.As BP Game Mode`))
  (bind _activehero (`/Game/Blueprints/BP_GameMode.ActiveHero` _as_bp_game_mode))
  (bind _asbp_enemy_base (cast `/Game/Blueprints/Enemies/BP_EnemyBase` TargetActor))
  (`GameplayStatics.ApplyDamage` _asbp_enemy_base (`KismetMathLibrary.Conv_IntToDouble` (`self.ZingerDamage`)) null null "/Game/Blueprints/DamageTypes/BP_ShockDamage.BP_ShockDamage_C")
  (`/Engine/EditorBlueprintResources/StandardMacros.IsValid` _asbp_enemy_base
    (:`Is Valid`
      (set `/Game/Blueprints/Enemies/BP_EnemyBase.Stunned` true _asbp_enemy_base)
      (set `/Game/Blueprints/Enemies/BP_EnemyBase.StunDuration` (`self.StunDuration`) _asbp_enemy_base)
      (`/Game/Blueprints/BP_GameMode.SetEnemyIntentions` _as_bp_game_mode)
      (`/Engine/EditorBlueprintResources/StandardMacros.DecrementInt` (`/Game/Blueprints/BP_GameMode.AlcoholPool` _as_bp_game_mode)
        (:`  `
          (`/Engine/EditorBlueprintResources/StandardMacros.DecrementInt` (`/Game/Blueprints/Heroes/BP_HeroBase.ActionPoints` _activehero)
            (:`  `
              (`/Game/Blueprints/Heroes/BP_HeroBase.SetActionPointsWidget` _activehero)
              (set `/Game/Blueprints/BP_GameMode.ActiveHero` null _as_bp_game_mode)
              (set `/Game/Blueprints/BP_PlayerController.SelectingTarget` false (`self.As BP Player Controller`))
              (`self.K2_DestroyActor`))))))))

(fn `UserConstructionScript`
  (`parent.UserConstructionScript`))