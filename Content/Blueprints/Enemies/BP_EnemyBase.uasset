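; Base enemy for what appears to be turn-based combat, with stamina and intent widgets and placeholder print-only choose and perform action events.
; Damage spawns a floating number at the projected screen position and passes through BPHealth; at zero or below, the enemy leaves the game state, has the game mode recheck enemies and intentions, then destroys itself.
; Tick copies current stamina to its widget, and SeducedIcon shows a red heart intent.
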(event `self.ReceiveTick`
  (params (DeltaSeconds :type "Float (single-precision)"))
  (`self.SetStaminaWidget`))

(event `self.ReceiveBeginPlay`
  (cast `/Game/Blueprints/BP_GameMode` (`GameplayStatics.GetGameMode`))
  (`SceneComponent.SetVisibility` (`self.IntentIcon`) false false)
  (`self.HideWidgetShadows`))

(event `ChooseAction`
  (if (not (`self.Stunned`))
    (`KismetSystemLibrary.PrintString` "I am going to attack")))

(event `self.PaperSprite.OnClicked`
  (params (TouchedComponent :type "PrimitiveComponent Object Reference") (ButtonPressed :type "Key Structure")))

(event `PerformAction`
  (`KismetSystemLibrary.PrintString` (`KismetStringLibrary.Concat_StrStr` (`KismetSystemLibrary.GetDisplayName` self) " performed an action")))

(event `/Game/Blueprints/Enemies/BPI_SetPosition.SetPosition`
  (params (Position :type "Actor Object Reference"))
  (set `self.Position` Position))

(event `self.ReceiveAnyDamage`
  (params (Damage :type "Float (single-precision)") (DamageType :type "DamageType Object Reference") (InstigatedBy :type "Controller Object Reference") (DamageCauser :type "Actor Object Reference"))
  ;[1 1 1] Take Damage - Archived (See BP_Health)
  (`self.ShowFloatingDamage` (`KismetMathLibrary.Round` Damage))
  (bind _currentstamina (`/Game/Blueprints/ActorComponents/BP_Health.DamageProcessing` (`self.BP_Health`) Damage))
  (if (<= _currentstamina 0)
    (bind _asbp_game_mode (cast `/Game/Blueprints/BP_GameMode` (`GameplayStatics.GetGameMode`)))
    (`/Game/Blueprints/BP_GameState.RemoveEnemy` (`/Game/Blueprints/BP_GameMode.As BP Game State` _asbp_game_mode) self)
    (`/Game/Blueprints/BP_GameMode.CheckEnemyPresence` _asbp_game_mode)
    (`/Game/Blueprints/BP_GameMode.SetEnemyIntentions` _asbp_game_mode)
    (`self.K2_DestroyActor`)))

(fn `HideWidgetShadows`
  (`PrimitiveComponent.SetCastShadow` (`self.StaminaWidget`) false)
  (`PrimitiveComponent.SetCastShadow` (`self.IntentIcon`) false))

(fn `SeducedIcon`
  (`SceneComponent.SetVisibility` (`self.IntentIcon`) true false)
  (bind _aswbp_enemy_intent (cast `/Game/UI/WBP_EnemyIntent` (`WidgetComponent.GetUserWidgetObject` (`self.IntentIcon`))))
  (bind _icon (`/Game/UI/WBP_EnemyIntent.Icon` _aswbp_enemy_intent))
  (bind (_imagesize _margin _tintcolor _resourceobject _drawas _tiling _mirroring) (break `SlateBrush` (`Image.Brush` _icon)))
  (`Image.SetBrush` _icon (make `SlateBrush` _imagesize _margin (make `SlateColor` (struct :`R` 1.0 :`A` 1.0)) "/Game/UI/Textures/Icons/Heart.Heart" _drawas _tiling _mirroring))
  (set `/Game/UI/WBP_EnemyIntent.Damage` 0 _aswbp_enemy_intent))

(fn `SetStaminaWidget`
  (bind _aswbp_enemy_stamina (cast `/Game/UI/WBP_EnemyStamina` (`WidgetComponent.GetUserWidgetObject` (`self.StaminaWidget`))))
  (set `/Game/UI/WBP_EnemyStamina.Stamina` (`/Game/Blueprints/ActorComponents/BP_Health.CurrentStamina` (`self.BP_Health`)) _aswbp_enemy_stamina))

(fn `ShowFloatingDamage`
  (params (Damage :type Integer))
  (bind _returnvalue (`|CreateWidget` "/Game/UI/WBP_FloatingDamage.WBP_FloatingDamage_C" null Damage))
  (`UserWidget.AddToViewport` _returnvalue 0)
  (`UserWidget.SetPositionInViewport` _returnvalue (`GameplayStatics.ProjectWorldToScreen` (`GameplayStatics.GetPlayerController` 0) (`self.K2_GetActorLocation` self)) true))

(fn `UserConstructionScript`)