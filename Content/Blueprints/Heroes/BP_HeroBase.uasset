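; Base actor for heroes in a stage-themed turn-based battle, spending action points on Pound, Throw Shade, Defend, Steal Spotlight and Pull Out.
; Stats load from DT_Heroes and seed stamina, Shield and Resolve, which absorb physical and mental damage before BPHealth; zero stamina sends the hero backstage.
; A timer-based click check separates selection from sending backstage, stage slots are tracked through StageLocation, and six-slot outfits are equipped as runtime-added components.
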(event `self.ReceiveBeginPlay`
  ;[1 1 1] Begin Play
  (bind _asbp_game_mode (cast `/Game/Blueprints/BP_GameMode` (`GameplayStatics.GetGameMode`)))
  (set `self.GameMode` _asbp_game_mode)
  (`self.SetHeroStats`)
  (`self.SetActionPointsWidget`)
  (`self.SetStartingStamina`)
  (`self.SetStartingShieldAndResolve`)
  (`self.HideClothingOnStart`))

(event `Pound`
  ;[1 1 1] Pound
  (bind _asbp_player_controller (cast `/Game/Blueprints/BP_PlayerController` (`GameplayStatics.GetPlayerController` 0)))
  (set `/Game/Blueprints/BP_PlayerController.SelectingTarget` true _asbp_player_controller)
  (set `/Game/Blueprints/BP_PlayerController.ActionTypes` "NewEnumerator0" _asbp_player_controller))

(event `self.ReceiveTick`
  (params (DeltaSeconds :type "Float (single-precision)"))
  ;[1 1 1] Tick
  (`self.SetStaminaWidget`)
  (`self.HighlightIfActiveHero`))

(event `/Game/Blueprints/Heroes/BPI_SetStageLocation.SetStageLocation`
  (params (Location :type "Actor Object Reference"))
  (bind _gamemode (`self.GameMode`))
  ;[1 1 1] Set Stage Location
  (bind _output_get (set `self.StageLocation` Location))
  (bind _asbp_spotlight (cast `/Game/Blueprints/Battlefield/StagePositions/BP_Spotlight` _output_get))
  (`KismetArrayLibrary.Array_RemoveItem` (`/Game/Blueprints/BP_GameMode.StageLocations` _gamemode) _asbp_spotlight)
  (`KismetSystemLibrary.Delay` 0.2)
  (`/Game/Blueprints/BP_GameMode.SetBackstageHeroCount` _gamemode)
  (`KismetSystemLibrary.PrintString` (`KismetSystemLibrary.GetClassDisplayName` (`GameplayStatics.GetObjectClass` (`self.StageLocation`)))))

(event `ThrowShade`
  ;[1 1 1] Throw Shade
  (bind _asbp_player_controller (cast `/Game/Blueprints/BP_PlayerController` (`GameplayStatics.GetPlayerController` 0)))
  (set `/Game/Blueprints/BP_PlayerController.SelectingTarget` true _asbp_player_controller)
  (set `/Game/Blueprints/BP_PlayerController.ActionTypes` "NewEnumerator1" _asbp_player_controller))

(event `Defend`
  ;[1 1 1] Defend
  (`self.IncreaseShield`)
  (`self.IncreaseResolve`)
  (`/Engine/EditorBlueprintResources/StandardMacros.DecrementInt` (`self.ActionPoints`)
    (:`  `
      (`self.SetActionPointsWidget`)
      (`/Game/Blueprints/BP_GameMode.CheckHeroActionsComplete` (`self.GameMode`)))))

(event `self.PaperSprite.OnClicked`
  (params (TouchedComponent :type "PrimitiveComponent Object Reference") (ButtonPressed :type "Key Structure"))
  (bind _gamemode (`self.GameMode`))
  ;[1 1 1] On Clicked
  (`self.DoubleClicked`
    (:`DoubleClicked`
      (if (`|EnumEquality` (`/Game/Blueprints/BP_GameMode.BattleState` _gamemode) "NewEnumerator0")
        (`self.AddHeroBackstage`)
        (`/Game/UI/WBP_HeroHUD.HideActionList` (`/Game/Blueprints/BP_GameMode.HUD` _gamemode))
        (bind _asbp_spotlight (cast `/Game/Blueprints/Battlefield/StagePositions/BP_Spotlight` (`self.StageLocation`)))
        (`KismetArrayLibrary.Array_Add` (`/Game/Blueprints/BP_GameMode.StageLocations` (`self.GameMode`)) _asbp_spotlight)))
    (:`SingleClicked`
      (if (`self.IsHeroOnstage`)
        (if (>= (`self.ActionPoints`) 1)
          (`self.HeroClicked`)
          (else
            (`KismetSystemLibrary.PrintString` "Hero has no action points")))))))

(event `StealSpotlight`
  ;[1 1 1] Steal Spotlight
  (if (> (`self.ActionPoints`) 0)
    (if (not (`self.IsHeroInSpotlight`))
      (bind _spotlighthero (`self.GetSpotlightHero`))
      (`self.SwitchToSpotlight` _spotlighthero)
      (`/Game/Blueprints/Heroes/BPI_SetStageLocation.SetStageLocation` _spotlighthero (`self.StageLocation`))
      (`self.SetHeroToSpotlight`))
    (else
      (`KismetSystemLibrary.PrintString` "No Action Point Available"))))

(event `PullOut`
  ;[1 1 1] Pull Out
  (if (> (`self.ActionPoints`) 0)
    (if (`self.IsHeroOnstage`)
      (bind _asbp_player_controller (cast `/Game/Blueprints/BP_PlayerController` (`GameplayStatics.GetPlayerController` 0)))
      (set `/Game/Blueprints/BP_PlayerController.SelectingHero` true _asbp_player_controller)
      (set `/Game/Blueprints/BP_PlayerController.ActionTypes` "NewEnumerator4" _asbp_player_controller))))

(event `self.ReceiveAnyDamage`
  (params (Damage :type "Float (single-precision)") (DamageType :type "DamageType Object Reference") (InstigatedBy :type "Controller Object Reference") (DamageCauser :type "Actor Object Reference"))
  (bind _returnvalue (`KismetMathLibrary.Round` Damage))
  ;[1 1 1] Take Damage
  (bind _damageout (`self.CalculateDamageReceived` _returnvalue DamageType))
  (`self.ShowFloatingDamage` _returnvalue)
  (bind _currentstamina (`/Game/Blueprints/ActorComponents/BP_Health.TakeDamage` (`self.BP_Health`) (`KismetMathLibrary.Conv_IntToDouble` _damageout)))
  (if (<= _currentstamina 0)
    (set `self.Pounded` true)
    (`self.AddHeroBackstage`)
    (`/Game/UI/WBP_HeroHUD.HideActionList` (`/Game/Blueprints/BP_GameMode.HUD` (`self.GameMode`)))
    (bind _asbp_spotlight (cast `/Game/Blueprints/Battlefield/StagePositions/BP_Spotlight` (`self.StageLocation`)))
    (`KismetArrayLibrary.Array_Add` (`/Game/Blueprints/BP_GameMode.StageLocations` (`self.GameMode`)) _asbp_spotlight)))

(fn `AddHeroBackstage`
  (bind _backstage (`/Game/Blueprints/BP_GameMode.Backstage` (`self.GameMode`)))
  (`self.K2_SetActorLocation` (`self.K2_GetActorLocation` _backstage))
  (set `/Game/Blueprints/BP_GameMode.ActiveHero` null (`self.GameMode`))
  (set `self.StageLocation` _backstage)
  (bind _returnvalue (`|CreateWidget` "/Game/UI/HeroBackstageWidgets/WBP_Hero.WBP_Hero_C" null (`self.HeroStats`)))
  (`/Game/UI/WBP_HeroHUD.AddHeroBackstage` (`/Game/Blueprints/BP_GameMode.HUD` (`self.GameMode`)) _returnvalue (`self.Pounded`)))

(fn `CalculateDamageReceived`
  (params (DamageIn :type Integer) (DamageType :type "DamageType Object Reference"))
  (returns (DamageOut :type Integer))
  (locals (`DamageCalculation (L)` :type Integer))
  (if (== (`GameplayStatics.GetObjectClass` DamageType) "/Game/Blueprints/Abilities/BP_MentalDamage.BP_MentalDamage_C")
    (if (>= (`local.DamageIn`) (`self.Resolve`))
      (bind _output_get (set `local.DamageCalculation (L)` (- (`local.DamageIn`) (`self.Resolve`))))
      (set `self.Resolve` 0)
      (return _output_get)
      (else
        (set `self.Resolve` (- (`self.Resolve`) (`local.DamageIn`)))
        (return 0)))
    (elif (>= (`local.DamageIn`) (`self.Shield`))
      (bind _output_get_2 (set `local.DamageCalculation (L)` (- (`local.DamageIn`) (`self.Shield`))))
      (set `self.Shield` 0)
      (return _output_get_2)
      (else
        (set `self.Shield` (- (`self.Shield`) (`local.DamageIn`)))
        (return 0)))))

(fn `CalculatePoundDamage`
  (returns (TotalDamage :type "Float (double-precision)"))
  (return (`KismetMathLibrary.Conv_IntToDouble` (+ 1 (`.Passion_5_34B7CC1B49BD8269316506884D42E651` (break `/Game/Blueprints/Heroes/F_HeroStats` (`self.HeroStats`)))))))

(fn `CalculateThrowShadeDamage`
  (returns (TotalDamage :type "Float (double-precision)"))
  (return (`KismetMathLibrary.Conv_IntToDouble` (+ 1 (`.Flamboyance_9_06BC7BDB4F46F89A0680F795480171AB` (break `/Game/Blueprints/Heroes/F_HeroStats` (`self.HeroStats`)))))))

(fn `DoubleClickTimer`
  (set `self.Clicked` false))

(fn `EquipAccessory`
  (params (Accessory :type "/Game/Blueprints/Outfits/ClothingClasses/BP_OutfitPiece Class Reference"))
  (set `/Game/Blueprints/Outfits/BP_Outfit.Accessory` Accessory (`self.Outfit`))
  (`SceneComponent.SetVisibility` (`self.Accessory`) true false)
  (bind _returnvalue (`|AddComponentByClass` (`/Game/Blueprints/Outfits/BP_Outfit.Accessory` (`self.Outfit`))))
  (bind _output_get (set `self.AccessoryObject` _returnvalue))
  (message `/Game/Blueprints/Outfits/BPI_EquipItem.EquipItem` _output_get (`/Game/Blueprints/BP_GameMode.ActiveHero` (`self.GameMode`))))

(fn `EquipBottom`
  (params (Bottom :type "/Game/Blueprints/Outfits/ClothingClasses/BP_OutfitPiece Class Reference"))
  (bind _output_get (set `/Game/Blueprints/Outfits/BP_Outfit.Bottom` Bottom (`self.Outfit`)))
  (bind _returnvalue (`|AddComponentByClass` _output_get))
  (bind _output_get_2 (set `self.BottomObject` _returnvalue))
  (message `/Game/Blueprints/Outfits/BPI_EquipItem.EquipItem` _output_get_2 (`/Game/Blueprints/BP_GameMode.ActiveHero` (`self.GameMode`)))
  (`SceneComponent.SetVisibility` (`self.Bottom`) true false))

(fn `EquipFeet`
  (params (Feet :type "/Game/Blueprints/Outfits/ClothingClasses/BP_OutfitPiece Class Reference"))
  (bind _output_get (set `/Game/Blueprints/Outfits/BP_Outfit.Feet` Feet (`self.Outfit`)))
  (bind _returnvalue (`|AddComponentByClass` _output_get))
  (bind _output_get_2 (set `self.FeetObject` _returnvalue))
  (message `/Game/Blueprints/Outfits/BPI_EquipItem.EquipItem` _output_get_2 (`/Game/Blueprints/BP_GameMode.ActiveHero` (`self.GameMode`)))
  (`SceneComponent.SetVisibility` (`self.Feet`) true false))

(fn `EquipFromCloset`
  (params (Item :type "/Game/Blueprints/Outfits/ClothingClasses/BP_OutfitPiece Class Reference"))
  (switch `/Game/Blueprints/Outfits/E_ItemSlots` (defaults `Object` Item)
    (:`NewEnumerator0`
      (`self.EquipHead` (`local.Item`)))
    (:`NewEnumerator1`
      (`self.EquipAccessory` (`local.Item`)))
    (:`NewEnumerator2`
      (`self.EquipTop` (`local.Item`)))
    (:`NewEnumerator4`
      (`self.EquipHands` (`local.Item`)))
    (:`NewEnumerator3`
      (`self.EquipBottom` (`local.Item`)))
    (:`NewEnumerator5`
      (`self.EquipFeet` (`local.Item`)))))

(fn `EquipHands`
  (params (Hands :type "/Game/Blueprints/Outfits/ClothingClasses/BP_OutfitPiece Class Reference"))
  (set `/Game/Blueprints/Outfits/BP_Outfit.Hands` Hands (`self.Outfit`))
  (`SceneComponent.SetVisibility` (`self.Hands`) true false)
  (bind _returnvalue (`|AddComponentByClass` (`/Game/Blueprints/Outfits/BP_Outfit.Hands` (`self.Outfit`))))
  (bind _output_get (set `self.HandsObject` _returnvalue))
  (message `/Game/Blueprints/Outfits/BPI_EquipItem.EquipItem` _output_get (`/Game/Blueprints/BP_GameMode.ActiveHero` (`self.GameMode`))))

(fn `EquipHead`
  (params (Head :type "/Game/Blueprints/Outfits/ClothingClasses/BP_OutfitPiece Class Reference"))
  (set `/Game/Blueprints/Outfits/BP_Outfit.Head` Head (`self.Outfit`))
  (`SceneComponent.SetVisibility` (`self.Head`) true false)
  (bind _returnvalue (`|AddComponentByClass` (`/Game/Blueprints/Outfits/BP_Outfit.Head` (`self.Outfit`))))
  (bind _output_get (set `self.HeadObject` _returnvalue))
  (message `/Game/Blueprints/Outfits/BPI_EquipItem.EquipItem` _output_get (`/Game/Blueprints/BP_GameMode.ActiveHero` (`self.GameMode`))))

(fn `EquipTop`
  (params (Top :type "/Game/Blueprints/Outfits/ClothingClasses/BP_OutfitPiece Class Reference"))
  (set `/Game/Blueprints/Outfits/BP_Outfit.Top` Top (`self.Outfit`))
  (`SceneComponent.SetVisibility` (`self.Top`) true false)
  (bind _returnvalue (`|AddComponentByClass` (`/Game/Blueprints/Outfits/BP_Outfit.Top` (`self.Outfit`))))
  (bind _output_get (set `self.TopObject` _returnvalue))
  (message `/Game/Blueprints/Outfits/BPI_EquipItem.EquipItem` _output_get (`/Game/Blueprints/BP_GameMode.ActiveHero` (`self.GameMode`))))

(fn `GetSpotlightHero`
  (returns (SpotlightHero :type "/Game/Blueprints/Heroes/BP_HeroBase Object Reference"))
  (bind _outactors (`GameplayStatics.GetAllActorsOfClass` "BP_HeroBase_C"))
  (for _array_element _outactors
    (if (== (`GameplayStatics.GetObjectClass` (`/Game/Blueprints/Heroes/BP_HeroBase.StageLocation` _array_element)) "/Game/Blueprints/Battlefield/StagePositions/BP_Spotlight.BP_Spotlight_C")
      (return _array_element))))

(fn `HeroClicked`
  (bind _gamemode (`self.GameMode`))
  (if (`|EnumEquality` (`/Game/Blueprints/BP_GameMode.BattleState` _gamemode) "NewEnumerator1")
    (set `/Game/Blueprints/BP_GameMode.ActiveHero` self _gamemode)
    (`/Game/UI/WBP_HeroHUD.ShowActionList` (`/Game/Blueprints/BP_GameMode.HUD` (`self.GameMode`)))))

(fn `HideClothingOnStart`
  (`SceneComponent.SetVisibility` (`self.Head`) false false)
  (`SceneComponent.SetVisibility` (`self.Accessory`) false false)
  (`SceneComponent.SetVisibility` (`self.Top`) false false)
  (`SceneComponent.SetVisibility` (`self.Hands`) false false)
  (`SceneComponent.SetVisibility` (`self.Bottom`) false false)
  (`SceneComponent.SetVisibility` (`self.Feet`) false false))

(fn `HighlightIfActiveHero`
  (bind _papersprite (`self.PaperSprite`))
  (if (== (`/Game/Blueprints/BP_GameMode.ActiveHero` (`self.GameMode`)) self)
    (`PaperSpriteComponent.SetSpriteColor` _papersprite (struct :`R` 0.4 :`G` 1.0 :`B` 0.4 :`A` 1.0))
    (else
      (`PaperSpriteComponent.SetSpriteColor` _papersprite (struct :`R` 1.0 :`G` 1.0 :`B` 1.0 :`A` 1.0)))))

(fn `IncreaseResolve`
  (set `self.Resolve` (+ (+ (`self.Resolve`) (`.Confidence_14_D6890B19473417451A3807B7E6EA1135` (break `/Game/Blueprints/Heroes/F_HeroStats` (`self.HeroStats`)))) 1)))

(fn `IncreaseShield`
  (set `self.Shield` (+ (+ (`self.Shield`) (`.Pride_7_538B5121425B92976EBD309C6BDA2B76` (break `/Game/Blueprints/Heroes/F_HeroStats` (`self.HeroStats`)))) 1)))

(fn `IsHeroInSpotlight`
  (returns (Spotlight :type Boolean))
  (return (== (`GameplayStatics.GetObjectClass` (`self.StageLocation`)) "/Game/Blueprints/Battlefield/StagePositions/BP_Spotlight.BP_Spotlight_C")))

(fn `IsHeroOnstage`
  (returns (IsOnStage :type Boolean))
  (bind _returnvalue (`GameplayStatics.GetObjectClass` (`self.StageLocation`)))
  (return (or (== _returnvalue "/Game/Blueprints/Battlefield/StagePositions/BP_Spotlight.BP_Spotlight_C") (== _returnvalue "/Game/Blueprints/Battlefield/StagePositions/BP_StageLeft.BP_StageLeft_C") (== _returnvalue "/Game/Blueprints/Battlefield/StagePositions/BP_StageRight.BP_StageRight_C"))))

(fn `IsSupporterAubergenie`
  (returns (IsAubergenie :type Boolean))
  (return (== (`/Game/Blueprints/BP_GameMode.Supporter` (`self.GameMode`)) "/Game/Blueprints/Supporters/BP_Aubergenie.BP_Aubergenie_C")))

(fn `Load Starting Outfit`
  (bind _outfit (`self.Outfit`))
  (bind (_head _accessory _top _hands _bottom _feet) (break `/Game/Blueprints/Outfits/F_EquippedOutfit` (`self.EquippedOutfit`)))
  (`|ExecutionSequence`
    (:`then_0`
      (set `/Game/Blueprints/Outfits/BP_Outfit.Head` _head _outfit))
    (:`then_1`
      (set `/Game/Blueprints/Outfits/BP_Outfit.Accessory` _accessory _outfit))
    (:`then_2`
      (set `/Game/Blueprints/Outfits/BP_Outfit.Top` _top _outfit))
    (:`then_3`
      (set `/Game/Blueprints/Outfits/BP_Outfit.Hands` _hands _outfit))
    (:`then_4`
      (set `/Game/Blueprints/Outfits/BP_Outfit.Bottom` _bottom _outfit))
    (:`then_5`
      (set `/Game/Blueprints/Outfits/BP_Outfit.Feet` _feet _outfit))))

(fn `MoveHeroBackstage`
  (`self.K2_SetActorLocation` (`self.K2_GetActorLocation` (`/Game/Blueprints/BP_GameMode.Backstage` (`self.GameMode`)))))

(fn `MoveHeroOnstage`
  (params (Location :type "Actor Object Reference"))
  (`self.K2_SetActorLocation` (`KismetMathLibrary.MakeVector` (.x (`self.K2_GetActorLocation` Location)) (.y (`self.K2_GetActorLocation` Location)) (+ (.z (`self.K2_GetActorLocation` Location)) 50.0)))
  (message `/Game/Blueprints/Heroes/BPI_SetStageLocation.SetStageLocation` self Location))

(fn `PulloutActionPointHandling`
  (if (not (`self.IsSupporterAubergenie`))
    (`/Engine/EditorBlueprintResources/StandardMacros.DecrementInt` (`self.ActionPoints`)
      (:`  `
        _)))
  (`self.SetActionPointsWidget`))

(fn `SetActionPointsWidget`
  (bind _aswbp_show_action_points (cast `/Game/UI/WBP_ShowActionPoints` (`WidgetComponent.GetUserWidgetObject` (`self.ActionPointWidget`))))
  (set `/Game/UI/WBP_ShowActionPoints.ActionPoints` (`self.ActionPoints`) _aswbp_show_action_points))

(fn `SetHeroStats`
  (bind _outrownames (`DataTableFunctionLibrary.GetDataTableRowNames` "/Game/Blueprints/Heroes/DT_Heroes.DT_Heroes"))
  (for _array_element _outrownames
    (if (== _array_element (`self.Name`))
      (bind _returnvalue (`|GetDataTableRow` "/Game/Blueprints/Heroes/DT_Heroes.DT_Heroes" _array_element)
        (:`then`
          (set `self.HeroStats` _returnvalue))))))

(fn `SetHeroToSpotlight`
  (bind _outactors (`GameplayStatics.GetAllActorsOfClass` "/Game/Blueprints/Battlefield/StagePositions/BP_Spotlight.BP_Spotlight_C"))
  (for _array_element _outactors
    (if (== (`GameplayStatics.GetObjectClass` _array_element) "/Game/Blueprints/Battlefield/StagePositions/BP_Spotlight.BP_Spotlight_C")
      (set `self.StageLocation` _array_element))))

(fn `SetStaminaWidget`
  (bind _aswbp_hero_stamina (cast `/Game/UI/WBP_HeroStamina` (`WidgetComponent.GetUserWidgetObject` (`self.StaminaWidget`))))
  (set `/Game/UI/WBP_HeroStamina.Stamina` (`/Game/Blueprints/ActorComponents/BP_Health.CurrentStamina` (`self.BP_Health`)) _aswbp_hero_stamina)
  (set `/Game/UI/WBP_HeroStamina.Shield` (`self.Shield`) _aswbp_hero_stamina)
  (set `/Game/UI/WBP_HeroStamina.Resolve` (`self.Resolve`) _aswbp_hero_stamina))

(fn `SetStartingShieldAndResolve`
  (bind (_name _herotype _basestamina _passion _pride _flamboyance _drama _fashion _confidence) (break `/Game/Blueprints/Heroes/F_HeroStats` (`self.HeroStats`)))
  (set `self.Shield` _pride)
  (set `self.Resolve` _confidence))

(fn `SetStartingStamina`
  (bind ((`BaseStamina_41_F1F684E24942F1500E0E05AC9A18556D` _basestamina) (`Pride_7_538B5121425B92976EBD309C6BDA2B76` _pride) (`Confidence_14_D6890B19473417451A3807B7E6EA1135` _confidence)) (break `/Game/Blueprints/Heroes/F_HeroStats` (`self.HeroStats`)))
  (set `/Game/Blueprints/ActorComponents/BP_Health.CurrentStamina` (+ (+ _pride _confidence) _basestamina) (`self.BP_Health`)))

(fn `ShowFloatingDamage`
  (params (Damage :type Integer))
  (bind _returnvalue (`|CreateWidget` "/Game/UI/WBP_FloatingDamage.WBP_FloatingDamage_C" null Damage))
  (`UserWidget.AddToViewport` _returnvalue 0)
  (`UserWidget.SetPositionInViewport` _returnvalue (`GameplayStatics.ProjectWorldToScreen` (`GameplayStatics.GetPlayerController` 0) (`self.K2_GetActorLocation` self)) true))

(fn `SwitchToSpotlight`
  (params (SpotlightHero :type "Actor Object Reference"))
  (locals (SpotlightLocation :type "Vector Structure" :default (0.0 0.0 0.0)) (CurrentLocation :type "Vector Structure" :default (0.0 0.0 0.0)))
  (set `local.SpotlightLocation` (`self.K2_GetActorLocation` SpotlightHero))
  (set `local.CurrentLocation` (`SceneComponent.K2_GetComponentLocation` (`self.DefaultSceneRoot`)))
  (`SceneComponent.K2_SetWorldLocation` (`self.DefaultSceneRoot`) (`local.SpotlightLocation`) false false)
  (`SceneComponent.K2_SetWorldLocation` (`Actor.RootComponent` SpotlightHero) (`local.CurrentLocation`) false false))

(fn `UserConstructionScript`)