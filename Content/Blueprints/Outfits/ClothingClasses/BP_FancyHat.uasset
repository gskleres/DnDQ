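; BP_FancyHat is a clothing item class for the outfit system that modifies the hero's Passion stat.
; EquipItem adds PassionModifier to the Passion field of the passed object's HeroStats struct, and UnequipItem subtracts it again.
; BeginPlay and Tick are disabled stubs.
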(event `/Game/Blueprints/Outfits/BPI_EquipItem.EquipItem`
  (params (NewParam :type "/Game/Blueprints/Heroes/BP_HeroBase Object Reference"))
  (bind _herostats (`/Game/Blueprints/Heroes/BP_HeroBase.HeroStats` NewParam))
  (bind _structout (setmembers `/Game/Blueprints/Heroes/F_HeroStats` :`StructRef` _herostats :`Passion` (+ (`.Passion_5_34B7CC1B49BD8269316506884D42E651` (break `/Game/Blueprints/Heroes/F_HeroStats` _herostats)) (`self.PassionModifier`))))
  (set `/Game/Blueprints/Heroes/BP_HeroBase.HeroStats` _structout NewParam))

(event `/Game/Blueprints/Outfits/BPI_EquipItem.UnequipItem`
  (params (NewParam :type "/Game/Blueprints/Heroes/BP_HeroBase Object Reference"))
  (bind _herostats (`/Game/Blueprints/Heroes/BP_HeroBase.HeroStats` NewParam))
  (bind _structout (setmembers `/Game/Blueprints/Heroes/F_HeroStats` :`StructRef` _herostats :`Passion` (- (`.Passion_5_34B7CC1B49BD8269316506884D42E651` (break `/Game/Blueprints/Heroes/F_HeroStats` _herostats)) (`self.PassionModifier`))))
  (set `/Game/Blueprints/Heroes/BP_HeroBase.HeroStats` _structout NewParam))