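; Harry Hole Pecker supporter that strikes a random non-boss enemy when a battle starts.
; On BattleStart it gathers every BP_EnemyBase actor and adds those not flagged as Boss to PossibleTargets.
; It applies damage to a random entry, with the amount taken from the CurrentStamina of a random target's BPHealth, apparently intended as an instant knockout.
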(event `self.BattleStart`
  (bind _outitem (`KismetArrayLibrary.Array_Random` (`self.PossibleTargets`)))
  (bind _outactors (`GameplayStatics.GetAllActorsOfClass` "/Game/Blueprints/Enemies/BP_EnemyBase.BP_EnemyBase_C"))
  (for _array_element _outactors
    (if (not (`/Game/Blueprints/Enemies/BP_EnemyBase.Boss` _array_element))
      (`KismetArrayLibrary.Array_Add` (`self.PossibleTargets`) _array_element)))
  (`GameplayStatics.ApplyDamage` _outitem (`KismetMathLibrary.Conv_IntToDouble` (`/Game/Blueprints/ActorComponents/BP_Health.CurrentStamina` (`/Game/Blueprints/Enemies/BP_EnemyBase.BP_Health` _outitem)))))

(fn `UserConstructionScript`
  (`parent.UserConstructionScript`))