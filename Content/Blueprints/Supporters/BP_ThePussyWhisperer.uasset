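; BP_ThePussyWhisperer is a battle supporter that, on round start, deals repeated damage to randomly picked enemies in the front column.
; SetFrontColumn checks enemy positions for the first occupied column, and GetEnemiesInFrontColumn adds that column's enemies to Targets.
; ReleaseThePussies loops back through a DoN capped at the battle round number, re-rolling a random index per target, so hits can fall short of that count.
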(event `self.BattleRoundStart`
  (set `self.PussyCount` (`/Game/Blueprints/BP_GameMode.BattleRound` (`self.As BP Game Mode`)))
  (`self.SetFrontColumn`)
  (`self.GetEnemiesInFrontColumn`)
  (`KismetSystemLibrary.PrintString` (`KismetStringLibrary.Conv_IntToString` (`KismetArrayLibrary.Array_Length` (`self.Targets`))))
  (`self.ReleaseThePussies`))

(fn `GetEnemiesInFrontColumn`
  (for _array_element (`/Game/Blueprints/BP_GameState.EnemyPositions` (`/Game/Blueprints/BP_GameMode.As BP Game State` (`self.As BP Game Mode`)))
    (bind (_enemy _type _row _column) (break `/Game/Blueprints/Battlefield/F_EnemyPosition` _array_element))
    (if (== _column (`self.FrontColumn`))
      (`KismetArrayLibrary.Array_Add` (`self.Targets`) _enemy))))

(fn `ReleaseThePussies`
  (bind _targets (`self.Targets`))
  (`/Engine/EditorBlueprintResources/StandardMacros.Do N` (`self.PussyCount`) :!label _label
    (:`Exit`
      (for (_array_element _array_index) _targets
        (if (== _array_index (`KismetMathLibrary.RandomIntegerInRange` 0 (- (`KismetArrayLibrary.Array_Length` _targets) 1)))
          (`GameplayStatics.ApplyDamage` _array_element (`self.Damage`) null self "/Game/Blueprints/Abilities/BP_DamageTypeBase.BP_DamageTypeBase_C")
          (goto _label))))))

(fn `SetFrontColumn`
  (locals (`Enemies (L)` :type "Array of /Game/Blueprints/Battlefield/F_EnemyPosition Structure") (`ValidTargets (L)` :type "Array of Actor Object Reference") (`Column (L)` :type Integer))
  (bind _output_get (set `local.Enemies (L)` (`/Game/Blueprints/BP_GameState.EnemyPositions` (`/Game/Blueprints/BP_GameMode.As BP Game State` (`self.As BP Game Mode`)))))
  (for _array_element _output_get
    (bind (_enemy _type _row _column) (break `/Game/Blueprints/Battlefield/F_EnemyPosition` _array_element))
    (if (== _column (`local.Column (L)`))
      (`KismetArrayLibrary.Array_Add` (`local.ValidTargets (L)`) _enemy)))
  (if (== (`KismetArrayLibrary.Array_Length` (`local.ValidTargets (L)`)) 0)
    (`/Engine/EditorBlueprintResources/StandardMacros.IncrementInt` (`local.Column (L)`)
      (:`  `
        (for _array_element_2 (`local.Enemies (L)`)
          (bind (_enemy_2 _type_2 _row_2 _column_2) (break `/Game/Blueprints/Battlefield/F_EnemyPosition` _array_element_2))
          (if (== _column_2 (`local.Column (L)`))
            (`KismetArrayLibrary.Array_Add` (`local.ValidTargets (L)`) _enemy_2)))
        (if (== (`KismetArrayLibrary.Array_Length` (`local.ValidTargets (L)`)) 0)
          (bind _result (`/Engine/EditorBlueprintResources/StandardMacros.IncrementInt` (`local.Column (L)`))
            (:`  `
              (set `self.FrontColumn` _result)))
          (else
            (set `self.FrontColumn` (`local.Column (L)`))))))
    (else
      (set `self.FrontColumn` (`local.Column (L)`)))))

(fn `UserConstructionScript`
  (`parent.UserConstructionScript`))