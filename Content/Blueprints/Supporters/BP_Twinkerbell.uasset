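; BP_Twinkerbell is a supporter Blueprint that brings back every hero in the Pounded state through one custom event.
; The event scans all BP_HeroBase actors and calls Comeback on those flagged Pounded.
; It then clears the Pounded flag on every WBP_Hero widget, including nested ones, without checking which hero each represents.
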(event `BringThemBitchesBack`
  (bind _outactors (`GameplayStatics.GetAllActorsOfClass` "/Game/Blueprints/Heroes/BP_HeroBase.BP_HeroBase_C"))
  (for _array_element _outactors
    (if (`/Game/Blueprints/Heroes/BP_HeroBase.Pounded` _array_element)
      (`/Game/Blueprints/Heroes/BP_HeroBase.Comeback` _array_element)))
  (bind _foundwidgets (`WidgetBlueprintLibrary.GetAllWidgetsOfClass` "/Game/UI/HeroBackstageWidgets/WBP_Hero.WBP_Hero_C" false))
  (for _array_element_2 _foundwidgets
    (set `/Game/UI/HeroBackstageWidgets/WBP_Hero.Pounded` false _array_element_2)))

(fn `UserConstructionScript`
  (`parent.UserConstructionScript`))