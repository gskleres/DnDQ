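; Game mode for the battle level that creates the battle UI and hands the battle result back to the game.
; On BeginPlay it creates the BattleRootUI widget, binds a handler to its battle-finished event and adds it to the viewport.
; EndBattle passes the result to the DnDQ game instance to end the current battle.
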(event `self.ReceiveBeginPlay`
  (`self.SetupUI`))

(fn `EndBattle`
  (params (In_BattleResult :type "/Game/Blueprints/BattleLevel/BattleResult_struct Structure"))
  (bind _asdn_dq_bpgi (cast `/Game/Blueprints/DnDQ_bpgi` (`GameplayStatics.GetGameInstance`)))
  (`/Game/Blueprints/DnDQ_bpgi.EndCurrentBattle` _asdn_dq_bpgi In_BattleResult))

(fn `SetupUI`
  (bind _returnvalue (`|CreateWidget` "/Game/Blueprints/BattleLevel/UI/BattleRootUI_bpw.BattleRootUI_bpw_C"))
  (bind _output_get (set `self.BattleUI` _returnvalue))
  (add `/Game/Blueprints/BattleLevel/UI/BattleRootUI_bpw.OnBattleFinished` _output_get (`|CreateDelegate` :!event `EndBattle`))
  (`UserWidget.AddToViewport` _output_get 0))

(fn `UserConstructionScript`)