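; Game instance for DnDQ that carries battle results between levels and holds a placeholder list of save games.
; On Init it spawns three SaveGameData actors with hard-coded timestamps and play times and adds them to FakeSaveGameList, a stand-in marked TODO for replacement.
; EndCurrentBattle stores the BattleResult and opens Game_Level, so the result persists across the level change.
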(event `self.ReceiveInit`
  ;[1 0 0] GJS TODO: this should be replaced withi anything resonable
  (`self.MakeFakeSaveDataList`))

(fn `EndCurrentBattle`
  (params (BattleResult :type "/Game/Blueprints/BattleLevel/BattleResult_struct Structure"))
  (set `self.BattleResult` BattleResult)
  (`GameplayStatics.OpenLevel` "Game_Level"))

(fn `MakeFakeSaveDataList`
  (bind _returnvalue (`KismetMathLibrary.MakeTransform` (0.0 0.0 0.0)))
  (`|ExecutionSequence`
    (:`then_0`
      (bind _returnvalue_2 (`|SpawnActorFromClass` "/Game/Blueprints/SaveGameData.SaveGameData_C" _returnvalue "Undefined" "OverrideRootScale" null null))
      (set `/Game/Blueprints/SaveGameData.TimestampOfLastSave` (`KismetMathLibrary.MakeDateTime` 2021 3 1 12 12 12) _returnvalue_2)
      (set `/Game/Blueprints/SaveGameData.GameTimeInSec` 33 _returnvalue_2)
      (`KismetArrayLibrary.Array_Add` (`self.FakeSaveGameList`) _returnvalue_2))
    (:`then_1`
      (bind _returnvalue_3 (`|SpawnActorFromClass` "/Game/Blueprints/SaveGameData.SaveGameData_C" _returnvalue "Undefined" "OverrideRootScale" null null))
      (set `/Game/Blueprints/SaveGameData.TimestampOfLastSave` (`KismetMathLibrary.MakeDateTime` 2021 3 9 9 3 9) _returnvalue_3)
      (set `/Game/Blueprints/SaveGameData.GameTimeInSec` 393 _returnvalue_3)
      (`KismetArrayLibrary.Array_Add` (`self.FakeSaveGameList`) _returnvalue_3))
    (:`then_2`
      (bind _returnvalue_4 (`|SpawnActorFromClass` "/Game/Blueprints/SaveGameData.SaveGameData_C" _returnvalue "Undefined" "OverrideRootScale" null null))
      (set `/Game/Blueprints/SaveGameData.TimestampOfLastSave` (`KismetMathLibrary.MakeDateTime` 2021 4 4 4 44 44) _returnvalue_4)
      (set `/Game/Blueprints/SaveGameData.GameTimeInSec` 4444 _returnvalue_4)
      (`KismetArrayLibrary.Array_Add` (`self.FakeSaveGameList`) _returnvalue_4))))