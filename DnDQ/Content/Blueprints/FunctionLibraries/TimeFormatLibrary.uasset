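; Blueprint function library that turns second counts and DateTime values into display strings.
; The seconds formatter builds colon-separated text, optionally hiding zero hours, and returns an error string for negatives.
; Its minutes field is total minutes, not wrapped at sixty, and is zero-padded only when hours are hidden.
; The DateTime formatter joins year-month-day@hour:minute without padding, dropping seconds rather than rounding.
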(fn `FormatHoursMinutesSecondsFromSeconds`
  (params (InNumSec :type Integer) (bHideHoursIfZero :type Boolean))
  (returns (OutString :type String))
  (bind _returnvalue (/ InNumSec 3600))
  (bind _returnvalue_2 (/ InNumSec 60))
  (bind _returnvalue_3 (mod InNumSec 60))
  (bind _returnvalue_4 (and (== _returnvalue 0) bHideHoursIfZero))
  (if (< InNumSec 0)
    (return "Error: NumSec < 0")
    (else
      (return (`KismetStringLibrary.Concat_StrStr` (`KismetMathLibrary.SelectString` "" (`KismetStringLibrary.Concat_StrStr` (`KismetStringLibrary.Conv_IntToString` _returnvalue) ":") _returnvalue_4) (`KismetStringLibrary.Concat_StrStr` (`KismetMathLibrary.SelectString` "0" "" (and _returnvalue_4 (< _returnvalue_2 10))) (`KismetStringLibrary.Conv_IntToString` _returnvalue_2) ":") (`KismetStringLibrary.Concat_StrStr` (`KismetMathLibrary.SelectString` "0" "" (< _returnvalue_3 10)) (`KismetStringLibrary.Conv_IntToString` _returnvalue_3)))))))

(fn `RoughFormatDateTime_RoundToMinutes`
  (params (InDateTime :type "DateTime Structure"))
  (returns (OutString :type String))
  (bind (_year _month _day _hour _minute) (`KismetMathLibrary.BreakDateTime` InDateTime))
  (return (`KismetStringLibrary.Concat_StrStr` (`KismetStringLibrary.Conv_IntToString` _year) "-" (`KismetStringLibrary.Conv_IntToString` _month) "-" (`KismetStringLibrary.Conv_IntToString` _day) " @ " (`KismetStringLibrary.Conv_IntToString` _hour) ":" (`KismetStringLibrary.Conv_IntToString` _minute))))