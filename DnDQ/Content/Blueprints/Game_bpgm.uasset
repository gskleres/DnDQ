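; Game mode that initialises a play session from saved data and runs the game clock.
; On BeginPlay it binds to the game state's data-loaded event, then passes it the save data held by the DnDQ game instance.
; StartGame creates the timer widget and starts a looping one-second timer.
; GameTimerTick increments the elapsed seconds stored on the game state and broadcasts a per-second dispatcher.
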(event `self.ReceiveBeginPlay`
  (bind _asdn_dq_bpgi (cast `/Game/Blueprints/DnDQ_bpgi` (`GameplayStatics.GetGameInstance`)))
  (bind _asgame_bpgs (cast `/Game/Blueprints/Game_bpgs` (`GameplayStatics.GetGameState`)))
  (set `self.GameStateRef` _asgame_bpgs)
  (add `/Game/Blueprints/Game_bpgs.OnGameDataLoaded` _asgame_bpgs (`|CreateDelegate` :!event `StartGame`))
  (`/Game/Blueprints/Game_bpgs.SetupGameState` _asgame_bpgs (`/Game/Blueprints/DnDQ_bpgi.SaveGameData` _asdn_dq_bpgi)))

(fn `GameTimerTick`
  (`/Engine/EditorBlueprintResources/StandardMacros.IncrementInt` (`/Game/Blueprints/Game_bpgs.GameTimeInSec` (`self.GameStateRef`))
    (:`  `
      (`self.OnGameTimerTickPerSecond`))))

(fn `StartGame`
  (bind _returnvalue (`KismetSystemLibrary.K2_SetTimerDelegate` (`|CreateDelegate` :!event `GameTimerTick`) 1.0 true))
  (set `self.GameTimer` _returnvalue)
  (bind _returnvalue_2 (`|CreateWidget` "/Game/UI/Game/GameTimer_bpw.GameTimer_bpw_C"))
  (`/Game/UI/Game/GameTimer_bpw.UpdateTimeDisplay` _returnvalue_2)
  (`UserWidget.AddToViewport` _returnvalue_2 0))

(fn `UserConstructionScript`)