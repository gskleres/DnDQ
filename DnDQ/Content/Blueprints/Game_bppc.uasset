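; Player controller for gameplay that toggles an escape menu widget with the Escape key.
; BeginPlay creates the ESC menu widget and shows the mouse cursor.
; Releasing Escape removes the menu if it is in the viewport, otherwise adds it and binds its quit and save click events.
; Quit exits the game, while the save handler is still empty.
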(event `self.ReceiveBeginPlay`
  (bind _returnvalue (`|CreateWidget` "/Game/UI/MainGame/ESC_Menu_bpw.ESC_Menu_bpw_C"))
  (set `self.EscapeMenu` _returnvalue)
  (set `self.bShowMouseCursor` true))

(event `InputAction|EscapeKey`
  (params (Key :type "Key Structure"))
  (bind _escapemenu (`self.EscapeMenu`))
  (:`Released`
    (if (`Widget.IsInViewport` _escapemenu)
      (`Widget.RemoveFromParent` _escapemenu)
      (else
        (`UserWidget.AddToViewport` _escapemenu 0)
        (add `/Game/UI/MainGame/ESC_Menu_bpw.OnQuitGameClicked` _escapemenu (delegate `HandleQuitGameClicked`))
        (add `/Game/UI/MainGame/ESC_Menu_bpw.OnSaveGameClicked` _escapemenu (delegate `HandleSaveGameClicked`))))))

(event `HandleQuitGameClicked`
  (`KismetSystemLibrary.QuitGame` null "Quit"))

(event `HandleSaveGameClicked`)

(fn `UserConstructionScript`)