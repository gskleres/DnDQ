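; Main menu game mode that shows the menu and launches or quits the game.
; On BeginPlay it clears the game instance's save data, creates the menu widget, binds its load, new game and quit events, and enables the mouse cursor.
; New game opens Game_level directly, while LoadGame first stores the given save data on the game instance, which carries it across the level change.
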(event `self.ReceiveBeginPlay`
  (bind _returnvalue (`GameplayStatics.GetPlayerController` 0))
  (`|ExecutionSequence`
    (:`then_0`
      ;[1 1 1] Reset save game data
      (bind _asdn_dq_bpgi (cast `/Game/Blueprints/DnDQ_bpgi` (`GameplayStatics.GetGameInstance`)))
      (set `/Game/Blueprints/DnDQ_bpgi.SaveGameData` null _asdn_dq_bpgi))
    (:`then_1`
      ;[1 1 1] Main Menu and its bindings
      (bind _returnvalue_2 (`|CreateWidget` "/Game/Blueprints/MainMenuLevel/UI/MainMenu_wbp.MainMenu_wbp_C"))
      (`UserWidget.AddToViewport` _returnvalue_2 0)
      (add `/Game/Blueprints/MainMenuLevel/UI/MainMenu_wbp.OnLoadClicked` _returnvalue_2 (`|CreateDelegate` :!event `LoadGame`))
      (add `/Game/Blueprints/MainMenuLevel/UI/MainMenu_wbp.OnNewGameClicked` _returnvalue_2 (delegate `HandleNewGame`))
      (add `/Game/Blueprints/MainMenuLevel/UI/MainMenu_wbp.OnQuitGameClicked` _returnvalue_2 (delegate `HandleQuitGame`))
      (set `PlayerController.bShowMouseCursor` true _returnvalue)
      (`WidgetBlueprintLibrary.SetInputMode_GameAndUIEx` _returnvalue _returnvalue_2 "DoNotLock" false))))

(event `HandleNewGame`
  ;[1 1 1] Main Menu and its bindings
  (`self.StartGame`))

(event `HandleQuitGame`
  ;[1 1 1] Main Menu and its bindings
  (`KismetSystemLibrary.QuitGame` null "Quit"))

(fn `LoadGame`
  (params (InSaveData :type "/Game/Blueprints/SaveGameData Object Reference"))
  (bind _asdn_dq_bpgi (cast `/Game/Blueprints/DnDQ_bpgi` (`GameplayStatics.GetGameInstance`)))
  (set `/Game/Blueprints/DnDQ_bpgi.SaveGameData` InSaveData _asdn_dq_bpgi)
  (`self.StartGame`))

(fn `StartGame`
  (`GameplayStatics.OpenLevel` "Game_level"))

(fn `UserConstructionScript`)