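; Game mode for the gameplay level that handles game startup, the play timer, saving and winning.
; BeginPlay passes the game instance's save data to the game state's setup and binds an event to its data-loaded dispatcher.
; A looping one-second timer drives the game-time counter and a per-second tick dispatcher.
; WinGame opens the win level, while SaveGame fills a save object and prints it without writing to a slot.
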(event `self.ReceiveBeginPlay`
  ;[1 1 1] Load the current save (it will be empty if it's a new game)
  (bind _asdn_dq_bpgi_interface (cast `/Game/Blueprints/DnDQ_bpgi_interface` (`GameplayStatics.GetGameInstance`)))
  (bind _out_savegame (`/Game/Blueprints/DnDQ_bpgi_interface.GetSaveData` _asdn_dq_bpgi_interface))
  (`/Engine/EditorBlueprintResources/StandardMacros.IsValid` _out_savegame
    (:`Is Valid`
      ;[1 1 1] Once the game state has finished loading, start the game!
      (bind _asgame_bpgs (cast `/Game/Blueprints/GameLevel/Game_bpgs` (`GameplayStatics.GetGameState`)))
      (set `self.GameStateRef` _asgame_bpgs)
      (add `/Game/Blueprints/GameLevel/Game_bpgs.OnGameDataLoaded` _asgame_bpgs (`|CreateDelegate` :!event `StartGame`))
      (`/Game/Blueprints/GameLevel/Game_bpgs.SetupGameState` _asgame_bpgs _out_savegame))))

(fn `GameTimerTick`
  (`/Engine/EditorBlueprintResources/StandardMacros.IncrementInt` (`/Game/Blueprints/GameLevel/Game_bpgs.GameTimeInSec` (`self.GameStateRef`))
    (:`  `
      (`self.OnGameTimerTickPerSecond`))))

(fn `SaveGame`
  (bind _returnvalue (`GameplayStatics.CreateSaveGameObject` "/Game/Blueprints/DnDQ_savegame.DnDQ_savegame_C"))
  (bind _asgame_bpgs (cast `/Game/Blueprints/GameLevel/Game_bpgs` (`GameplayStatics.GetGameState`)))
  (set `/Game/Blueprints/DnDQ_savegame.TimestampOfLastSave` (struct) _returnvalue)
  (bind _output_get (set `/Game/Blueprints/DnDQ_savegame.GameTimeInSec` (`/Game/Blueprints/GameLevel/Game_bpgs.GameTimeInSec` _asgame_bpgs) _returnvalue))
  (`KismetSystemLibrary.PrintString` (`KismetStringLibrary.Concat_StrStr` "Saved game w/ " (`KismetStringLibrary.Conv_IntToString` _output_get)) true true (struct :`G` 0.66 :`B` 1.0 :`A` 1.0) 10.0))

(fn `StartGame`
  (bind _returnvalue (`KismetSystemLibrary.K2_SetTimerDelegate` (`|CreateDelegate` :!event `GameTimerTick`) 1.0 true))
  (set `self.GameTimer` _returnvalue))

(fn `UserConstructionScript`)

(fn `WinGame`
  (`GameplayStatics.OpenLevel` "Win_level"))