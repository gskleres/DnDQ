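; Player controller for the game level that manages the timer HUD, escape menu and cheat panel.
; On BeginPlay it creates the three widgets, shows the timer and mouse cursor, and sets game-only input.
; Input actions toggle the menu and cheat panel.
; Widget events route to handlers that quit, or call SaveGame and WinGame on the Game_bpgm game mode.
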(event `self.ReceiveBeginPlay`
  (bind _returnvalue (`|CreateWidget` "/Game/Blueprints/GameLevel/UI/GameESC_Menu_bpw.GameESC_Menu_bpw_C"))
  (set `self.EscapeMenu` _returnvalue)
  (set `self.bShowMouseCursor` true)
  (`|ExecutionSequence`
    (:`then_0`
      (bind _returnvalue_2 (`|CreateWidget` "/Game/Blueprints/GameLevel/UI/GameTimer_bpw.GameTimer_bpw_C"))
      (`/Game/Blueprints/GameLevel/UI/GameTimer_bpw.UpdateTimeDisplay` _returnvalue_2)
      (`UserWidget.AddToViewport` _returnvalue_2 0))
    (:`then_1`
      (`self.SetupCheatUI`))
    (:`then_2`
      (`WidgetBlueprintLibrary.SetInputMode_GameOnly` self))))

(event `InputAction|EscapeKey`
  (params (Key :type "Key Structure"))
  (bind _escapemenu (`self.EscapeMenu`))
  (:`Released`
    (if (`Widget.IsInViewport` _escapemenu)
      (`Widget.RemoveFromParent` _escapemenu)
      (else
        (`UserWidget.AddToViewport` _escapemenu 0)
        (add `/Game/Blueprints/GameLevel/UI/GameESC_Menu_bpw.OnQuitGameClicked` _escapemenu (delegate `HandleQuitGameClicked`))
        (add `/Game/Blueprints/GameLevel/UI/GameESC_Menu_bpw.OnSaveGameClicked` _escapemenu (delegate `HandleSaveGameClicked`))))))

(event `HandleQuitGameClicked`
  (`KismetSystemLibrary.QuitGame` null "Quit"))

(event `HandleSaveGameClicked`
  (bind _asgame_bpgm (cast `/Game/Blueprints/GameLevel/Game_bpgm` (`GameplayStatics.GetGameMode`)))
  (`/Game/Blueprints/GameLevel/Game_bpgm.SaveGame` _asgame_bpgm))

(event `InputAction|EnableCheatUI`
  (params (Key :type "Key Structure"))
  (bind _cheatui (`self.CheatUI`))
  (:`Released`
    (if (`Widget.IsInViewport` (`self.CheatUI`))
      (`Widget.RemoveFromParent` _cheatui)
      (else
        (`UserWidget.AddToViewport` _cheatui 0)))))

(fn `HandleCheatWinGame`
  (bind _asgame_bpgm (cast `/Game/Blueprints/GameLevel/Game_bpgm` (`GameplayStatics.GetGameMode`)))
  (`/Game/Blueprints/GameLevel/Game_bpgm.WinGame` _asgame_bpgm))

(fn `SetupCheatUI`
  (bind _returnvalue (`|CreateWidget` "/Game/Blueprints/GameLevel/UI/GameCheatUI_bpw.GameCheatUI_bpw_C"))
  (bind _output_get (set `self.CheatUI` _returnvalue))
  (`|ExecutionSequence`
    (:`then_0`
      (add `/Game/Blueprints/GameLevel/UI/GameCheatUI_bpw.CheatWinGameClicked` _output_get (`|CreateDelegate` :!event `HandleCheatWinGame`)))))

(fn `UserConstructionScript`)